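; BP_Elevator is a one-shot elevator that starts when an actor tagged Player enters its Box trigger.
; The Elevator_Time timeline's ElevationTrack drives lerps that move the StaticMesh and a referenced RectLight toward separate target locations.
; Each lerp starts from the current location rather than a cached start, so motion compounds every update.
; When the timeline finishes, the Box is destroyed to prevent retriggering.
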(event `self.Box.OnComponentBeginOverlap`
  (params (OverlappedComponent :type "PrimitiveComponent Object Reference") (OtherActor :type "Actor Object Reference") (OtherComp :type "PrimitiveComponent Object Reference") (OtherBodyIndex :type Integer) (bFromSweep :type Boolean) (SweepResult :type "HitResult Structure (by ref)"))
  (bind _staticmesh (`self.StaticMesh`))
  (bind _rootcomponent (`Actor.RootComponent` (`self.RectLight`)))
  ;[1 1 1] Comment
  (if (`self.ActorHasTag` OtherActor "Player")
    (bind (_direction _elevation_track) (`Timeline|Elevator_Time` :!via `PlayFromStart`)
      (:`Update`
        (`SceneComponent.K2_SetWorldLocation` _staticmesh (`KismetMathLibrary.VLerp` (`SceneComponent.K2_GetComponentLocation` _staticmesh) (`self.NewLocation`) _elevation_track) false false)
        (`SceneComponent.K2_SetWorldLocation` _rootcomponent (`KismetMathLibrary.VLerp` (`SceneComponent.K2_GetComponentLocation` _rootcomponent) (`self.New Location Rect`) _elevation_track) false false))
      (:`Finished`
        (`ActorComponent.K2_DestroyComponent` (`self.Box`))))))

(fn `UserConstructionScript`)