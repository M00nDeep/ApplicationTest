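; Breakable block that spawns a random physics pickup and hides itself when the player hits it with an upward vertical impact normal.
; Dropped coins raise the maximum coin count through the GameState.
; A visibility snapshot from BeginPlay and checkpoints drives restoring the block on player death, which also retracts that coin increment.
; The broken state saves and loads by ObjectIndex.
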(event `self.ReceiveBeginPlay`
  ;[1 1 1] BeginPlay Event
  (set `self.DroppedItemClass` null)
  (message `/Game/Custom_0/Blueprints/GameplayFramework/SaveSystem/BPI_Persistent.I_RequestLoad` (`GameplayStatics.GetGameInstance`) self)
  (`self.PopulateResetStruct`)
  ;;[0.08999 0.7582 1] Bind events to reset dispatchers
  (bind _asbp_game_state_main (cast `/Game/Custom_0/Blueprints/GameplayFramework/WorldProgression/BP_GameStateMain` (`GameplayStatics.GetGameState`)))
  (add `/Game/Custom_0/Blueprints/GameplayFramework/WorldProgression/BP_GameStateMain.PlayerDied` _asbp_game_state_main (delegate `InternalReset`))
  (bind _asbp_player_state_main (cast `/Game/Custom_0/Blueprints/GameplayFramework/BP_PlayerStateMain` (`GameplayStatics.GetPlayerState` 0)))
  (add `/Game/Custom_0/Blueprints/GameplayFramework/BP_PlayerStateMain.CheckpointReached` _asbp_player_state_main (delegate `InternalCheckpointReached`)))

(event `InternalReset`
  (bind _resetstruct_visible_ (break `/Game/Custom_0/Blueprints/GameplayFramework/ResetValuesStructs/BPS_ResetBlock` (`self.ResetStruct`)))
  ;[1 1 1] BeginPlay Event
  ;;[0.08999 0.7582 1] Bind events to reset dispatchers
  (if _resetstruct_visible_
    (`self.ResetBlock`)
    (if (== (`self.DroppedItemClass`) "/Game/Custom_0/Blueprints/Objects/PickUpables/BP_DroppedCoin.BP_DroppedCoin_C")
      (message `/Game/Custom_0/Blueprints/GameplayFramework/WorldProgression/BPI_UpdateWorldQuest.I_RemoveMaximumCoin` (`GameplayStatics.GetGameState`))
      (set `self.DroppedItemClass` null))))

(event `InternalCheckpointReached`
  ;[1 1 1] BeginPlay Event
  ;;[0.08999 0.7582 1] Bind events to reset dispatchers
  (`self.PopulateResetStruct`))

(event `DropItem`
  ;[1 1 1] Drop Item and check if an eventually active Coin Quest needs to be updated
  (bind _output_get (set `self.DroppedItemClass` (`KismetArrayLibrary.Array_Random` (`self.DropArray`))))
  (if (`KismetSystemLibrary.IsValidClass` _output_get)
    (bind _returnvalue (`|SpawnActorFromClass` _output_get (`self.SpawnObjectFuncUtility`) "AdjustIfPossibleButAlwaysSpawn" "MultiplyWithRoot" null (`GameplayStatics.GetPlayerPawn` 0)))
    (`self.CheckForMoreCoins`)
    (bind _asbp_pickup_base (cast `/Game/Custom_0/Blueprints/Objects/PickUpables/BP_PickupBase` _returnvalue))
    (set `/Game/Custom_0/Blueprints/Objects/PickUpables/BP_PickupBase.NeedSave?` false _asbp_pickup_base)
    (`PrimitiveComponent.SetSimulatePhysics` (`/Game/Custom_0/Blueprints/Objects/PickUpables/BP_PickupBase.Object` _asbp_pickup_base) true)))

(event `DestroyBlock`
  ;[1 1 1] Hide Block
  (`PrimitiveComponent.SetSimulatePhysics` (`self.StaticMesh`) false)
  (`SceneComponent.SetHiddenInGame` (`self.StaticMesh`) true true)
  (`PrimitiveComponent.SetCollisionEnabled` (`self.Box`) "NoCollision")
  (`PrimitiveComponent.SetCollisionEnabled` (`self.StaticMesh`) "NoCollision"))

(event `ResetBlock`
  ;[1 1 1] Reset Block
  (`SceneComponent.SetHiddenInGame` (`self.StaticMesh`) false false)
  (`PrimitiveComponent.SetCollisionEnabled` (`self.Box`) "QueryAndPhysics")
  (`PrimitiveComponent.SetCollisionEnabled` (`self.StaticMesh`) "QueryAndPhysics"))

(event `self.StaticMesh.OnComponentHit`
  (params (HitComponent :type "PrimitiveComponent Object Reference") (OtherActor :type "Actor Object Reference") (OtherComp :type "PrimitiveComponent Object Reference") (NormalImpulse :type "Vector Structure") (Hit :type "HitResult Structure (by ref)"))
  ;[1 1 1] Check for correct Hit with Static Mesh
  (if (`self.ActorHasTag` OtherActor "Player")
    (if (`self.CheckNormalDirection` (.x (`.ImpactNormal` (`GameplayStatics.BreakHitResult` Hit))) (.y (`.ImpactNormal` (`GameplayStatics.BreakHitResult` Hit))) (.z (`.ImpactNormal` (`GameplayStatics.BreakHitResult` Hit))))
      (set `self.AlreadyBroken` true)
      (`self.DropItem`)
      (`self.DestroyBlock`))))

(event `/Game/Custom_0/Blueprints/GameplayFramework/SaveSystem/BPI_Saveable.I_SaveData`
  (params (SaveGameRef :type "/Game/Custom_0/Blueprints/GameplayFramework/SaveSystem/BP_Save Object Reference"))
  ;[0 0.1261 1] Saving System
  (`BlueprintMapLibrary.Map_Add` (`/Game/Custom_0/Blueprints/GameplayFramework/SaveSystem/BP_Save.BlockStructData` SaveGameRef) (`self.ObjectIndex`) (make `/Game/Custom_0/Blueprints/GameplayFramework/SaveSystem/StructDatas/BPS_BlocksStruct` (`self.AlreadyBroken`))))

(event `/Game/Custom_0/Blueprints/GameplayFramework/SaveSystem/BPI_Saveable.I_LoadData`
  (params (SaveGameRef :type "/Game/Custom_0/Blueprints/GameplayFramework/SaveSystem/BP_Save Object Reference"))
  (bind (_value _returnvalue) (`BlueprintMapLibrary.Map_Find` (`/Game/Custom_0/Blueprints/GameplayFramework/SaveSystem/BP_Save.BlockStructData` SaveGameRef) (`self.ObjectIndex`)))
  ;[0 0.1261 1] Saving System
  (if _returnvalue
    (bind _output_get (set `self.AlreadyBroken` (break `/Game/Custom_0/Blueprints/GameplayFramework/SaveSystem/StructDatas/BPS_BlocksStruct` _value)))
    (if _output_get
      (`self.DestroyBlock`))))

(fn `CheckNormalDirection`
  (params (X :type "Float (double-precision)") (Y :type "Float (double-precision)") (Z :type "Float (double-precision)"))
  (returns (Out :type Boolean))
  (return (and (<= (`KismetMathLibrary.Abs` X) 0.1) (<= (`KismetMathLibrary.Abs` Y) 0.1) (>= Z 0.1))))

(fn `PopulateResetStruct`
  (set `self.ResetStruct` (make `/Game/Custom_0/Blueprints/GameplayFramework/ResetValuesStructs/BPS_ResetBlock` (`SceneComponent.IsVisible` (`self.StaticMesh`)))))

(fn `SpawnObjectFuncUtility`
  (returns (ReturnValue :type "Transform Structure"))
  (bind (_returnvalue_x _returnvalue_y _returnvalue_z) (`KismetMathLibrary.BreakVector` (`SceneComponent.K2_GetComponentLocation` (`self.Box`))))
  (return (`KismetMathLibrary.MakeTransform` (`KismetMathLibrary.MakeVector` _returnvalue_x _returnvalue_y (+ _returnvalue_z (`self.ZOffset`))) (`self.K2_GetActorRotation`))))

(fn `UserConstructionScript`)