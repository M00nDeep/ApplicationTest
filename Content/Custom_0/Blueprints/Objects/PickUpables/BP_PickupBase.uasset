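; Base Blueprint for pickups, triggered when a Player-tagged actor overlaps its Box, with PickUp and AlreadyPickedUp as override points.
; The picked-up flag saves and loads through the save game by ObjectIndex.
; When NeedSave is set, it requests loading and snapshots visibility on start and at checkpoints, re-showing the pickup on player death if it was visible.
; Helper events toggle visibility and collision, with hiding also stopping physics.
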(event `self.ReceiveBeginPlay`
  ;[1 1 1] BeginPlay Event
  (if (`self.NeedSave?`)
    (message `/Game/Custom_0/Blueprints/GameplayFramework/SaveSystem/BPI_Persistent.I_RequestLoad` (`GameplayStatics.GetGameInstance`) self)
    (`self.PopulateResetStruct`)
    ;;[0.2436 0.7141 1] Bind to reset dispatchers
    (bind _asbp_game_state_main (cast `/Game/Custom_0/Blueprints/GameplayFramework/WorldProgression/BP_GameStateMain` (`GameplayStatics.GetGameState`)))
    (add `/Game/Custom_0/Blueprints/GameplayFramework/WorldProgression/BP_GameStateMain.PlayerDied` _asbp_game_state_main (delegate `InternalReset`))
    (bind _asbp_player_state_main (cast `/Game/Custom_0/Blueprints/GameplayFramework/BP_PlayerStateMain` (`GameplayStatics.GetPlayerState` 0)))
    (add `/Game/Custom_0/Blueprints/GameplayFramework/BP_PlayerStateMain.CheckpointReached` _asbp_player_state_main (delegate `InternalCheckpointReached`))))

(event `InternalReset`
  (bind _resetstruct_visible_ (break `/Game/Custom_0/Blueprints/GameplayFramework/ResetValuesStructs/BPS_ResetPickup` (`self.ResetStruct`)))
  ;[1 1 1] BeginPlay Event
  ;;[0.2436 0.7141 1] Bind to reset dispatchers
  (if _resetstruct_visible_
    (`self.ShowYourself`)))

(event `InternalCheckpointReached`
  ;[1 1 1] BeginPlay Event
  ;;[0.2436 0.7141 1] Bind to reset dispatchers
  (`self.PopulateResetStruct`))

(event `HideYourself`
  ;[1 1 1] Hide yourself
  (`PrimitiveComponent.SetSimulatePhysics` (`self.Object`) false)
  (`PrimitiveComponent.SetCollisionEnabled` (`self.Object`) "NoCollision")
  (`PrimitiveComponent.SetCollisionEnabled` (`self.Box`) "NoCollision")
  (`SceneComponent.SetHiddenInGame` (`self.Object`) true true))

(event `ShowYourself`
  ;[1 1 1] Reset pickup
  (`PrimitiveComponent.SetCollisionEnabled` (`self.Object`) "QueryAndPhysics")
  (`PrimitiveComponent.SetCollisionEnabled` (`self.Box`) "QueryAndPhysics")
  (`SceneComponent.SetHiddenInGame` (`self.Object`) false false))

(event `self.Box.OnComponentBeginOverlap`
  (params (OverlappedComponent :type "PrimitiveComponent Object Reference") (OtherActor :type "Actor Object Reference") (OtherComp :type "PrimitiveComponent Object Reference") (OtherBodyIndex :type Integer) (bFromSweep :type Boolean) (SweepResult :type "HitResult Structure (by ref)"))
  ;[1 1 1] BeginOverlap
  (if (`self.ActorHasTag` OtherActor "Player")
    (`self.PickUp`)))

(event `AlreadyPickedUp`
  ;[1 1 1] Base methods to override
)

(event `PickUp`
  ;[1 1 1] Base methods to override
  (set `self.PickedUp` true))

(event `/Game/Custom_0/Blueprints/GameplayFramework/SaveSystem/BPI_Saveable.I_SaveData`
  (params (SaveGameRef :type "/Game/Custom_0/Blueprints/GameplayFramework/SaveSystem/BP_Save Object Reference"))
  ;[0.04598 0.07154 1] Save System
  (`BlueprintMapLibrary.Map_Add` (`/Game/Custom_0/Blueprints/GameplayFramework/SaveSystem/BP_Save.PickupStructData` SaveGameRef) (`self.ObjectIndex`) (make `/Game/Custom_0/Blueprints/GameplayFramework/SaveSystem/StructDatas/BPS_PickupData` (`self.PickedUp`))))

(event `/Game/Custom_0/Blueprints/GameplayFramework/SaveSystem/BPI_Saveable.I_LoadData`
  (params (SaveGameRef :type "/Game/Custom_0/Blueprints/GameplayFramework/SaveSystem/BP_Save Object Reference"))
  (bind (_value _returnvalue) (`BlueprintMapLibrary.Map_Find` (`/Game/Custom_0/Blueprints/GameplayFramework/SaveSystem/BP_Save.PickupStructData` SaveGameRef) (`self.ObjectIndex`)))
  ;[0.04598 0.07154 1] Save System
  (if _returnvalue
    (bind _output_get (set `self.PickedUp` (break `/Game/Custom_0/Blueprints/GameplayFramework/SaveSystem/StructDatas/BPS_PickupData` _value)))
    (if _output_get
      (`self.AlreadyPickedUp`))))

(fn `PopulateResetStruct`
  (set `self.ResetStruct` (make `/Game/Custom_0/Blueprints/GameplayFramework/ResetValuesStructs/BPS_ResetPickup` (`SceneComponent.IsVisible` (`self.Object`)))))

(fn `UserConstructionScript`)