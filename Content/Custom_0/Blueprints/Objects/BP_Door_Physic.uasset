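; Physics-driven door that stays locked until a specific quest is completed.
; On BeginPlay it locks the swing of two physics constraints and binds to quest progression on BP_GameStateMain.
; When the completed quest matches GateFromQuest, both constraints switch to limited swing so the door can move.
; A player-tagged actor entering the TriggerClose volume locks both constraints again at zero angle.
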(event `self.ReceiveBeginPlay`
  (`PhysicsConstraintComponent.SetAngularSwing1Limit` (`self.PhysicsConstraint1`) "ACM_Locked" 0.0)
  (`PhysicsConstraintComponent.SetAngularSwing1Limit` (`self.PhysicsConstraint`) "ACM_Locked" 0.0)
  (bind _asbp_game_state_main (cast `/Game/Custom_0/Blueprints/GameplayFramework/WorldProgression/BP_GameStateMain` (`GameplayStatics.GetGameState`)))
  (add `/Game/Custom_0/Blueprints/GameplayFramework/WorldProgression/BP_GameStateMain.QuestProgression` _asbp_game_state_main (delegate `QuestWasCompleted`)))

(event `QuestWasCompleted`
  (params (QuestCompleted :type "/Game/Custom_0/Blueprints/GameplayFramework/WorldProgression/E_WorldQuests Enum" :default "NewEnumerator0"))
  (if (`|EnumEquality` QuestCompleted (`self.GateFromQuest`))
    (`PhysicsConstraintComponent.SetAngularSwing1Limit` (`self.PhysicsConstraint1`) "ACM_Limited" 100.0)
    (`PhysicsConstraintComponent.SetAngularSwing1Limit` (`self.PhysicsConstraint`) "ACM_Limited" 100.0)))

(event `self.TriggerClose.OnComponentBeginOverlap`
  (params (OverlappedComponent :type "PrimitiveComponent Object Reference") (OtherActor :type "Actor Object Reference") (OtherComp :type "PrimitiveComponent Object Reference") (OtherBodyIndex :type Integer) (bFromSweep :type Boolean) (SweepResult :type "HitResult Structure (by ref)"))
  (if (`self.ActorHasTag` OtherActor "Player")
    (`PhysicsConstraintComponent.SetAngularSwing1Limit` (`self.PhysicsConstraint1`) "ACM_Locked" 0.0)
    (`PhysicsConstraintComponent.SetAngularSwing1Limit` (`self.PhysicsConstraint`) "ACM_Locked" 0.0)))

(fn `UserConstructionScript`)