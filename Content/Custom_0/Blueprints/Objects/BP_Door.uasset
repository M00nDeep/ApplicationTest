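; Double-gate door that swings away from the player on overlap once unlocked by completing its assigned quest, turning green when unlocked.
; A timeline mirrors the rotation across both pivots, while a looping timer polls for unlocking if the player is waiting in the trigger.
; On exit it either closes after a retriggerable delay or destroys its trigger.
; Unlock state is saved and loaded per object index through interface events.
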(event `self.ReceiveBeginPlay`
  ;[1 1 1] Begin Play - Load Data if there are any
  (message `/Game/Custom_0/Blueprints/GameplayFramework/SaveSystem/BPI_Persistent.I_RequestLoad` (`GameplayStatics.GetGameInstance`) self)
  (bind _asbp_game_state_main (cast `/Game/Custom_0/Blueprints/GameplayFramework/WorldProgression/BP_GameStateMain` (`GameplayStatics.GetGameState`)))
  (add `/Game/Custom_0/Blueprints/GameplayFramework/WorldProgression/BP_GameStateMain.QuestProgression` _asbp_game_state_main (delegate `QuestWasCompleted`)))

(event `QuestWasCompleted`
  (params (QuestCompleted :type "/Game/Custom_0/Blueprints/GameplayFramework/WorldProgression/E_WorldQuests Enum" :default "NewEnumerator0"))
  ;[1 1 1] Begin Play - Load Data if there are any
  (if (`|EnumEquality` QuestCompleted (`self.GateFromQuest`))
    (set `self.CanOpen?` true)
    (`self.SetOpenGateColors`)))

(event `Open`
  ;[1 0.1354 0.1354] Open/Close
  (if (not (`self.TotallyOpened`))
    (if (and (`TimelineComponent.IsPlaying` (`self.OpenTimeline`)) (!= (`self.UsableEndRot`) (`self.EndRot`) :`ErrorTolerance` 0.01))
      (`KismetSystemLibrary.RetriggerableDelay` (`TimelineComponent.GetPlaybackPosition` (`self.OpenTimeline`))))
    (set `self.UsableStartRot` (`self.StartRot`))
    (set `self.UsableEndRot` (`self.EndRot`))
    (`TimelineComponent.Stop` (`self.OpenTimeline`))
    (bind (_direction _alpha) (`Timeline|OpenTimeline` :!label _label)
      (:`Update`
        (bind _returnvalue (`KismetMathLibrary.RLerp` (`self.UsableStartRot`) (`self.UsableEndRot`) _alpha))
        (`SceneComponent.K2_SetRelativeRotation` (`self.PivotL`) _returnvalue false false)
        (`SceneComponent.K2_SetRelativeRotation` (`self.PivotR`) (* _returnvalue -1.0) false false))
      (:`Finished`
        (if (`|EnumEquality` _direction "Forward")
          (set `self.TotallyOpened` true))))))

(event `Close`
  ;[1 0.1354 0.1354] Open/Close
  (set `self.TotallyOpened` false)
  (`TimelineComponent.Stop` (`self.OpenTimeline`))
  (goto _label :!via `Reverse`))

(event `self.Box.OnComponentBeginOverlap`
  (params (OverlappedComponent :type "PrimitiveComponent Object Reference") (OtherActor :type "Actor Object Reference") (OtherComp :type "PrimitiveComponent Object Reference") (OtherBodyIndex :type Integer) (bFromSweep :type Boolean) (SweepResult :type "HitResult Structure (by ref)"))
  ;[0.2379 0.7249 1] BeginOverlap - Check If can be opened and set Values
  (if (`self.ActorHasTag` OtherActor "Player")
    (set `self.OverlappingFlag` true)
    (if (> (.x (`KismetMathLibrary.LessLess_VectorRotator` (- (`self.K2_GetActorLocation`) (`self.K2_GetActorLocation` (`GameplayStatics.GetPlayerPawn` 0))) (`self.K2_GetActorRotation`))) 0.0)
      (set `self.EndRot` (struct :`Yaw` 90.0))
      (else
        (set `self.EndRot` (struct :`Yaw` -90.0))))
    (if (`self.CanOpen?`)
      (`self.Open`)
      (else
        (bind _returnvalue (`KismetSystemLibrary.K2_SetTimerDelegate` (delegate `CheckForKey`) 0.1 true))
        (set `self.OpenTimerHandle` _returnvalue)))))

(event `CheckForKey`
  ;[0.2379 0.7249 1] BeginOverlap - Check If can be opened and set Values
  (if (`self.CanOpen?`)
    (`KismetSystemLibrary.K2_ClearAndInvalidateTimerHandle` (`self.OpenTimerHandle`))
    (`self.Open`)))

(event `self.Box.OnComponentEndOverlap`
  (params (OverlappedComponent :type "PrimitiveComponent Object Reference") (OtherActor :type "Actor Object Reference") (OtherComp :type "PrimitiveComponent Object Reference") (OtherBodyIndex :type Integer))
  ;[0.2379 0.7249 1] EndOverlap - Close
  (if (`self.ActorHasTag` OtherActor "Player")
    (set `self.OverlappingFlag` false)
    (if (`self.CanCloseItself?`)
      (`KismetSystemLibrary.K2_ClearAndInvalidateTimerHandle` (`self.OpenTimerHandle`))
      (`KismetSystemLibrary.RetriggerableDelay` (`self.CloseGateDelay`))
      (if (not (`self.OverlappingFlag`))
        (`self.Close`))
      (else
        (`ActorComponent.K2_DestroyComponent` (`self.Box`))
        (`KismetSystemLibrary.K2_ClearAndInvalidateTimerHandle` (`self.OpenTimerHandle`))))))

(event `/Game/Custom_0/Blueprints/GameplayFramework/SaveSystem/BPI_Saveable.I_SaveData`
  (params (SaveGameRef :type "/Game/Custom_0/Blueprints/GameplayFramework/SaveSystem/BP_Save Object Reference"))
  ;[0.0237 0 1] Saving System
  (`BlueprintMapLibrary.Map_Add` (`/Game/Custom_0/Blueprints/GameplayFramework/SaveSystem/BP_Save.DoorStructData` SaveGameRef) (`self.ObjectIndex`) (make `/Game/Custom_0/Blueprints/GameplayFramework/SaveSystem/StructDatas/BPS_DoorStruct` (`self.CanOpen?`))))

(event `/Game/Custom_0/Blueprints/GameplayFramework/SaveSystem/BPI_Saveable.I_LoadData`
  (params (SaveGameRef :type "/Game/Custom_0/Blueprints/GameplayFramework/SaveSystem/BP_Save Object Reference"))
  (bind (_value _returnvalue) (`BlueprintMapLibrary.Map_Find` (`/Game/Custom_0/Blueprints/GameplayFramework/SaveSystem/BP_Save.DoorStructData` SaveGameRef) (`self.ObjectIndex`)))
  ;[0.0237 0 1] Saving System
  (if _returnvalue
    (bind _output_get (set `self.CanOpen?` (break `/Game/Custom_0/Blueprints/GameplayFramework/SaveSystem/StructDatas/BPS_DoorStruct` _value)))
    (if _output_get
      (`self.SetOpenGateColors`))))

(fn `SetOpenGateColors`
  (`PrimitiveComponent.SetMaterial` (`self.GateL`) 0 "/Game/Custom_0/Assets/Materials/M_Green.M_Green")
  (`PrimitiveComponent.SetMaterial` (`self.GateR`) 0 "/Game/Custom_0/Assets/Materials/M_Green.M_Green")
  (return))

(fn `UserConstructionScript`)