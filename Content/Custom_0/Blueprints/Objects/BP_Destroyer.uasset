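; BP_Destroyer is a trigger actor that removes a set of placed actors when the Player enters its box.
; The overlap starts a delayed loop that destroys MeshToDestroy entries one at a time, advancing Index until it exceeds the array length.
; Between removals it sends IDestroyNPCMessage with ToDestroy to the referenced NPC.
; Its ISendCanShoot interface function always returns false.
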(event `self.Box.OnComponentBeginOverlap`
  (params (OverlappedComponent :type "PrimitiveComponent Object Reference") (OtherActor :type "Actor Object Reference") (OtherComp :type "PrimitiveComponent Object Reference") (OtherBodyIndex :type Integer) (bFromSweep :type Boolean) (SweepResult :type "HitResult Structure (by ref)"))
  (bind _meshtodestroy (`self.MeshToDestroy`))
  (bind _index (`self.Index`))
  (if (`self.ActorHasTag` OtherActor "Player")
    (`self.K2_DestroyActor` (`|GetArrayItem` _meshtodestroy _index) :!label _label)
    (`/Engine/EditorBlueprintResources/StandardMacros.IncrementInt` _index
      (:`  `
        (if (not (> _index (`KismetArrayLibrary.Array_Length` _meshtodestroy)))
          (message `/Game/Custom_0/Blueprints/NPCs/BPI_Dialogues.I_DestroyNPC` (`self.BP_NPCRef`) (`self.To Destroy?`))
          (`KismetSystemLibrary.Delay` 0.2)
          (goto _label))))))

(fn `I_SendCanShoot`
  (returns (`CanShoot?` :type Boolean))
  (return false))

(fn `UserConstructionScript`)