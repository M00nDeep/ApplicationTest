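; BP_NPCs_Finale is the finale NPC Blueprint, which ends its main-quest conversation and shows the final quest screen.
; When its dialogue widget is invalidated, it clears the widget reference and resets the dialogue index.
; On the first invalidation only, guarded by AlreadyTalked, it sends the MainQuest end-conversation interface message to the GameState and adds WBP_FinalQuest to the viewport.
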(event `self.InvalidateWidget`
  (set `self.WBP_NPC_DialogueRef` null)
  (set `self.DialogueIndex` -1)
  (if (not (`self.AlreadyTalked`))
    (message `/Game/Custom_0/Blueprints/GameplayFramework/WorldProgression/BPI_UpdateWorldQuest.I_EndConversation` (`GameplayStatics.GetGameState`) (`self.MainQuest?`))
    (set `self.AlreadyTalked` true)
    (bind _returnvalue (`|CreateWidget` "/Game/Custom_0/Blueprints/Widgets/WBP_FinalQuest.WBP_FinalQuest_C" (`GameplayStatics.GetPlayerController` 0)))
    (`UserWidget.AddToViewport` _returnvalue 0)))

(fn `UserConstructionScript`
  (`parent.UserConstructionScript`))