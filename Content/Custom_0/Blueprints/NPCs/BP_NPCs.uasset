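; BP_NPCs is an NPC Blueprint that shows an overlay material while the player is in its trigger zone and runs linear, multi-line dialogue.
; Each Talk call advances an index through DialogueText, lazily creating and updating a dialogue widget, which trigger overlaps show or hide.
; When dialogue runs out, it resets and, the first time only, sends MainQuest to the GameState through an end-conversation interface message.
; An interface event can destroy the NPC.
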(event `self.TriggerZone.OnComponentBeginOverlap`
  (params (OverlappedComponent :type "PrimitiveComponent Object Reference") (OtherActor :type "Actor Object Reference") (OtherComp :type "PrimitiveComponent Object Reference") (OtherBodyIndex :type Integer) (bFromSweep :type Boolean) (SweepResult :type "HitResult Structure (by ref)"))
  ;[1 1 1] BeginOverlap - Set Overlay Material - Add Widget
  (if (`self.ActorHasTag` OtherActor "Player")
    (`MeshComponent.SetOverlayMaterial` (`self.Mesh`) "/Game/Custom_0/Assets/Materials/MI_OverlayMaterial.MI_OverlayMaterial")
    (if (< (`self.DialogueIndex`) (`KismetArrayLibrary.Array_Length` (`self.DialogueText`)))
      (bind _wbp_npc_dialogueref (`self.WBP_NPC_DialogueRef`)
        (:`then`
          (`UserWidget.AddToViewport` _wbp_npc_dialogueref 0))
        (:`else`))
      (else
        (`self.InvalidateWidget`)))))

(event `self.TriggerZone.OnComponentEndOverlap`
  (params (OverlappedComponent :type "PrimitiveComponent Object Reference") (OtherActor :type "Actor Object Reference") (OtherComp :type "PrimitiveComponent Object Reference") (OtherBodyIndex :type Integer))
  ;[1 1 1] EndOverlap - ReSet Overlay Material None - Remove Widget
  (if (`self.ActorHasTag` OtherActor "Player")
    (`MeshComponent.SetOverlayMaterial` (`self.Mesh`) null)
    (bind _wbp_npc_dialogueref (`self.WBP_NPC_DialogueRef`)
      (:`then`
        (`Widget.RemoveFromParent` _wbp_npc_dialogueref))
      (:`else`
        _))
    (if (not (< (`self.DialogueIndex`) (`KismetArrayLibrary.Array_Length` (`self.DialogueText`))))
      (`self.InvalidateWidget`))))

(event `/Game/Custom_0/Blueprints/NPCs/BPI_Dialogues.Talk`
  (bind _dialogueindex (`self.DialogueIndex`))
  ;[1 1 1] Talk System
  (`/Engine/EditorBlueprintResources/StandardMacros.IncrementInt` _dialogueindex
    (:`  `
      (if (< _dialogueindex (`KismetArrayLibrary.Array_Length` (`self.DialogueText`)))
        (`self.WBP_NPC_DialogueRef`
          (:`then`
            _)
          (:`else`
            (bind _returnvalue (`|CreateWidget` "/Game/Custom_0/Blueprints/NPCs/WBP_NPC_Dialogue.WBP_NPC_Dialogue_C" (`GameplayStatics.GetPlayerController` 0)))
            (bind _output_get (set `self.WBP_NPC_DialogueRef` _returnvalue))
            (`UserWidget.AddToViewport` _output_get 0)))
        (`TextBlock.SetText` (`/Game/Custom_0/Blueprints/NPCs/WBP_NPC_Dialogue.DialogueText` (`self.WBP_NPC_DialogueRef`)) (`KismetTextLibrary.Conv_StringToText` (`|GetArrayItem` (`self.DialogueText`) (`self.DialogueIndex`))))
        (else
          (`Widget.RemoveFromParent` (`self.WBP_NPC_DialogueRef`))
          (`self.InvalidateWidget`))))))

(event `InvalidateWidget`
  (set `self.WBP_NPC_DialogueRef` null)
  (set `self.DialogueIndex` -1)
  (if (not (`self.AlreadyTalked`))
    (message `/Game/Custom_0/Blueprints/GameplayFramework/WorldProgression/BPI_UpdateWorldQuest.I_EndConversation` (`GameplayStatics.GetGameState`) (`self.MainQuest?`))
    (set `self.AlreadyTalked` true)))

(event `/Game/Custom_0/Blueprints/NPCs/BPI_Dialogues.I_DestroyNPC`
  (params (`ToDestroy?` :type Boolean))
  (if `ToDestroy?`
    (`self.K2_DestroyActor`)))

(fn `UserConstructionScript`)