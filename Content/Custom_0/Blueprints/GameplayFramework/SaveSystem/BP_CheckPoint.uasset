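; BP_CheckPoint is a checkpoint actor that turns its flag green and triggers a save when the player reaches it.
; Overlapping its box marks it used, destroys the box, requests a save through the GameInstance and notifies PlayerState, all via interface messages.
; It requests a load on BeginPlay and persists its used flag in the save's TriggerStructData map by ObjectIndex, reapplying the used state when loaded.
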(event `self.ReceiveBeginPlay`
  ;[1 1 1] Even checkpoint needs save
  (message `/Game/Custom_0/Blueprints/GameplayFramework/SaveSystem/BPI_Persistent.I_RequestLoad` (`GameplayStatics.GetGameInstance`) self))

(event `self.Box.OnComponentBeginOverlap`
  (params (OverlappedComponent :type "PrimitiveComponent Object Reference") (OtherActor :type "Actor Object Reference") (OtherComp :type "PrimitiveComponent Object Reference") (OtherBodyIndex :type Integer) (bFromSweep :type Boolean) (SweepResult :type "HitResult Structure (by ref)"))
  ;[1 1 1] Checkpoint reached - notify PlayerState
  (if (`self.ActorHasTag` OtherActor "Player")
    (`self.CheckpointUsed`)
    (message `/Game/Custom_0/Blueprints/GameplayFramework/SaveSystem/BPI_Persistent.I_RequestSave` (`GameplayStatics.GetGameInstance`) true)
    (message `/Game/Custom_0/Blueprints/GameplayFramework/BPI_NotifyPlayerState.I_NotifyCheckpointReached` (`GameplayStatics.GetPlayerState` 0))))

(event `/Game/Custom_0/Blueprints/GameplayFramework/SaveSystem/BPI_Saveable.I_SaveData`
  (params (SaveGameRef :type "/Game/Custom_0/Blueprints/GameplayFramework/SaveSystem/BP_Save Object Reference"))
  ;[0.04928 0.08844 1] Save System
  (`BlueprintMapLibrary.Map_Add` (`/Game/Custom_0/Blueprints/GameplayFramework/SaveSystem/BP_Save.TriggerStructData` SaveGameRef) (`self.ObjectIndex`) (make `/Game/Custom_0/Blueprints/GameplayFramework/SaveSystem/StructDatas/BPS_TriggerStruct` (`self.AlreadyUsed`))))

(event `/Game/Custom_0/Blueprints/GameplayFramework/SaveSystem/BPI_Saveable.I_LoadData`
  (params (SaveGameRef :type "/Game/Custom_0/Blueprints/GameplayFramework/SaveSystem/BP_Save Object Reference"))
  (bind (_value _returnvalue) (`BlueprintMapLibrary.Map_Find` (`/Game/Custom_0/Blueprints/GameplayFramework/SaveSystem/BP_Save.TriggerStructData` SaveGameRef) (`self.ObjectIndex`)))
  ;[0.04928 0.08844 1] Save System
  (if _returnvalue
    (bind _output_get (set `self.AlreadyUsed` (break `/Game/Custom_0/Blueprints/GameplayFramework/SaveSystem/StructDatas/BPS_TriggerStruct` _value)))
    (if _output_get
      (`self.CheckpointUsed`))))

(fn `CheckpointUsed`
  (set `self.AlreadyUsed` true)
  (`PrimitiveComponent.SetMaterial` (`self.Flag`) 0 "/Game/Custom_0/Assets/Materials/M_Green.M_Green")
  (`ActorComponent.K2_DestroyComponent` (`self.Box`))
  (return))

(fn `UserConstructionScript`)