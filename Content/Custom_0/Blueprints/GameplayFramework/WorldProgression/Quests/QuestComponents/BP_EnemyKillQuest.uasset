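; BP_EnemyKillQuest is a quest that tracks enemy kills toward a target supplied by the game state.
; On BeginPlay it gets the target through an interface message, creates the enemy quest HUD widget and sends it the total.
; Update and reset events raise or lower the count by one and refresh the widget.
; Reaching the target on an update removes the widget and reports completion to BP_GameStateMain.
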(event `self.ReceiveBeginPlay`
  ;[1 1 1] BeginPlay Event - Initialize quest
  (`|ExecutionSequence`
    (:`then_0`
      (set `self.QuestType` "NewEnumerator1")
      (bind (_globalquesttype _coinstocollect _enemiestokill) (message `/Game/Custom_0/Blueprints/GameplayFramework/WorldProgression/BPI_UpdateWorldQuest.I_SendQuestSpecifics` (`GameplayStatics.GetGameState`)))
      (set `self.EnemiesToKill` _enemiestokill)
      (set `self.WidgetClass` "/Game/Custom_0/Blueprints/Widgets/WBP_EnemyQuestHUD.WBP_EnemyQuestHUD_C"))
    (:`then_1`
      (`self.AddQuestWidget` self)
      (message `/Game/Custom_0/Blueprints/Widgets/BPI_SendDataToWidget.I_SendTotalEnemiesQuest` (`self.WidgetRef`) (`self.EnemiesToKill`)))))

(event `EnemiesUpdate`
  ;[1 1 1] Add single enemy count killed
  (bind _result (`/Engine/EditorBlueprintResources/StandardMacros.IncrementInt` (`self.CurrentEnemiesKilled`))
    (:`  `
      (message `/Game/Custom_0/Blueprints/Widgets/BPI_SendDataToWidget.I_SendCurrentKilledEnemiesQuest` (`self.WidgetRef`) _result)
      (`self.CheckQuestCompletition`))))

(event `EnemiesReset`
  ;[1 1 1] Reset single enemy count killed
  (if (> (`self.CurrentEnemiesKilled`) 0)
    (bind _result (`/Engine/EditorBlueprintResources/StandardMacros.DecrementInt` (`self.CurrentEnemiesKilled`))
      (:`  `
        (message `/Game/Custom_0/Blueprints/Widgets/BPI_SendDataToWidget.I_SendCurrentKilledEnemiesQuest` (`self.WidgetRef`) _result)))))

(event `self.CheckQuestCompletition`
  ;[1 1 1] Check Quest Completition
  (if (>= (`self.CurrentEnemiesKilled`) (`self.EnemiesToKill`))
    (`self.RemoveQuestWidget`)
    (bind _asbp_game_state_main (cast `/Game/Custom_0/Blueprints/GameplayFramework/WorldProgression/BP_GameStateMain` (`GameplayStatics.GetGameState`)))
    (`/Game/Custom_0/Blueprints/GameplayFramework/WorldProgression/BP_GameStateMain.QuestCompleted` _asbp_game_state_main (`self.QuestType`))))