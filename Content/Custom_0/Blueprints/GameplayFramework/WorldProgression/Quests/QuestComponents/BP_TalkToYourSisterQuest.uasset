(event `self.ReceiveBeginPlay`
  ;[1 1 1] BeginPlay - Initialize quest
  (`|ExecutionSequence`
    (:`then_0`
      (set `self.QuestType` "NewEnumerator3")
      (bind (_globalquesttype _coinstocollect _enemiestokill _talktoyoursister) (message `/Game/Custom_0/Blueprints/GameplayFramework/WorldProgression/BPI_UpdateWorldQuest.I_SendQuestSpecifics` (`GameplayStatics.GetGameState`)))
      (set `self.Talk to Your Sister` _talktoyoursister)
      (set `self.WidgetClass` "/Game/Custom_0/Blueprints/Widgets/WBP_TalkToYourSisterHUD.WBP_TalkToYourSisterHUD_C"))
    (:`then_1`
      (`self.AddQuestWidget` self))))

(event `self.CheckQuestCompletition`
  ;[1 1 1] Check Quest completition
  (if (`self.Talk to Your Sister`)
    (`self.RemoveQuestWidget`)
    (bind _asbp_game_state_main (cast `/Game/Custom_0/Blueprints/GameplayFramework/WorldProgression/BP_GameStateMain` (`GameplayStatics.GetGameState`)))
    (`/Game/Custom_0/Blueprints/GameplayFramework/WorldProgression/BP_GameStateMain.QuestCompleted` _asbp_game_state_main (`self.QuestType`))))