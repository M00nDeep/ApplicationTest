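; BP_TalkToNPCQuest is a quest component for talk-to-NPC objectives, handling the quest's HUD and completion.
; On BeginPlay it sets its quest type, gets the target NPC name from the game state by interface message, then adds WBP_TalkToNPCHUD and passes it the name.
; A QuestCompleted event flagged as valid removes the widget and reports the quest type to BP_GameStateMain.
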(event `self.ReceiveBeginPlay`
  ;[1 1 1] BeginPlay - Initialize quest
  (`|ExecutionSequence`
    (:`then_0`
      (set `self.QuestType` "NewEnumerator3")
      (bind (_globalquesttype _coinstocollect _enemiestokill _npcname) (message `/Game/Custom_0/Blueprints/GameplayFramework/WorldProgression/BPI_UpdateWorldQuest.I_SendQuestSpecifics` (`GameplayStatics.GetGameState`)))
      (set `self.NPCName` _npcname)
      (set `self.WidgetClass` "/Game/Custom_0/Blueprints/Widgets/WBP_TalkToNPCHUD.WBP_TalkToNPCHUD_C"))
    (:`then_1`
      (`self.AddQuestWidget` self)
      (message `/Game/Custom_0/Blueprints/Widgets/BPI_SendDataToWidget.I_SendNPCName` (`self.WidgetRef`) (`self.NPCName`)))))

(event `self.CheckQuestCompletition`
  ;[1 1 1] Check Quest completition
  (`self.RemoveQuestWidget`)
  (bind _asbp_game_state_main (cast `/Game/Custom_0/Blueprints/GameplayFramework/WorldProgression/BP_GameStateMain` (`GameplayStatics.GetGameState`)))
  (`/Game/Custom_0/Blueprints/GameplayFramework/WorldProgression/BP_GameStateMain.QuestCompleted` _asbp_game_state_main (`self.QuestType`)))

(event `QuestCompleted`
  (params (ValidForQuestCompletition :type Boolean))
  ;[1 1 1] Check Quest completition
  (if ValidForQuestCompletition
    (`self.CheckQuestCompletition`)))