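; Game State that drives the world's linear quest progression, saving and loading the current quest and triggering end game at the last stage.
; Each quest enum value adds a talk, kill or coin quest component, configured from DT_QuestSpecifics by row index.
; Interface events forward coin, enemy and conversation updates to the active component.
; Completing a quest destroys its component, then advances the enum once no quest components remain.
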(event `self.ReceiveBeginPlay`
  ;[1 1 1] Begin Play - Load Current Quest and Define it
  (message `/Game/Custom_0/Blueprints/GameplayFramework/SaveSystem/BPI_Persistent.I_RequestLoad` (`GameplayStatics.GetGameInstance`) self)
  (`self.DefineCurrentQuest` (`self.CurrentQuest`)))

(event `/Game/Custom_0/Blueprints/GameplayFramework/WorldProgression/BPI_UpdateWorldQuest.I_SetQuestOnNewMap`
  ;[1 1 1] Assign Correct quests based on Enum
  (`KismetSystemLibrary.DelayUntilNextTick`)
  (bind _output_get (set `self.CurrentQuest` "NewEnumerator2"))
  (`self.TotalResetQuest`)
  (`self.DefineCurrentQuest` _output_get))

(event `TotalResetQuest`
  (for _array_element (`self.K2_GetComponentsByClass` self "/Game/Custom_0/Blueprints/GameplayFramework/WorldProgression/Quests/QuestComponents/BP_BaseQuestComponent.BP_BaseQuestComponent_C")
    (`/Engine/EditorBlueprintResources/StandardMacros.IsValid` _array_element
      (:`Is Valid`
        (`/Game/Custom_0/Blueprints/GameplayFramework/WorldProgression/Quests/QuestComponents/BP_BaseQuestComponent.RemoveQuestWidget` _array_element)
        (`ActorComponent.K2_DestroyComponent` _array_element)))))

(event `/Game/Custom_0/Blueprints/GameplayFramework/WorldProgression/BPI_UpdateWorldQuest.I_SetFinalQuest`
  ;[1 1 1] Assign Correct quests based on Enum
  (`KismetSystemLibrary.DelayUntilNextTick`)
  (bind _output_get (set `self.CurrentQuest` "NewEnumerator6"))
  (`self.TotalResetQuest`)
  (`self.DefineCurrentQuest` _output_get))

(event `DefineCurrentQuest`
  (params (CurrentQuest :type "/Game/Custom_0/Blueprints/GameplayFramework/WorldProgression/E_WorldQuests Enum" :default "NewEnumerator0"))
  ;[1 1 1] Assign Correct quests based on Enum
  (switch `/Game/Custom_0/Blueprints/GameplayFramework/WorldProgression/E_WorldQuests` CurrentQuest
    (:`NewEnumerator0`
      (bind _returnvalue (`AddComponent|NODE_AddBP_TalkToYourSisterQuest-0`))
      (set `self.TalkToNPCQuest` _returnvalue))
    (:`NewEnumerator1`
      (bind _returnvalue_2 (`AddComponent|NODE_AddBP_EnemyKillQuest-0`))
      (set `self.KillingEnemiesQuest` _returnvalue_2))
    (:`NewEnumerator2`
      (bind _returnvalue_3 (`AddComponent|NODE_AddBP_CollectCoinQuest-1`))
      (set `self.CoinCollectionQuest` _returnvalue_3))
    (:`NewEnumerator4`
      (bind _returnvalue_4 (`AddComponent|NODE_AddBP_EnemyKillQuest-2`))
      (set `self.KillingEnemiesQuest` _returnvalue_4))
    (:`NewEnumerator5`
      (bind _returnvalue_5 (`AddComponent|NODE_AddBP_TalkToNPCQuest-0`))
      (set `self.TalkToNPCQuest` _returnvalue_5))
    (:`NewEnumerator6`
      (bind _returnvalue_6 (`AddComponent|NODE_AddBP_TalkToNPCQuest-1`))
      (set `self.TalkToNPCQuest` _returnvalue_6))
    (:`NewEnumerator3`
      (`self.EndGame`))))

(event `/Game/Custom_0/Blueprints/GameplayFramework/WorldProgression/BPI_UpdateWorldQuest.I_ResetQuests`
  ;[1 1 1] Assign Correct quests based on Enum
  (`KismetSystemLibrary.DelayUntilNextTick`)
  (bind _output_get (set `self.CurrentQuest` "NewEnumerator0"))
  (`self.TotalResetQuest`)
  (`self.DefineCurrentQuest` _output_get))

(event `QuestCompleted`
  (params (QuestTypeCompleted :type "/Game/Custom_0/Blueprints/GameplayFramework/WorldProgression/Quests/E_QuestTypes Enum" :default "NewEnumerator0"))
  ;[1 1 1] Quest was completed - notify everyone and remove relative component
  (`self.RemoveCurrentQuestData` QuestTypeCompleted)
  (bind _allassignedquestcompleted_ (`self.CheckIfAllQuestWereCompleted`))
  (if _allassignedquestcompleted_
    (`self.QuestProgression` (`self.CurrentQuest`))
    (`self.QuestWasCompleted`)
    (`self.DefineCurrentQuest` (`self.CurrentQuest`))))

(event `/Game/Custom_0/Blueprints/GameplayFramework/SaveSystem/BPI_Saveable.I_SaveData`
  (params (SaveGameRef :type "/Game/Custom_0/Blueprints/GameplayFramework/SaveSystem/BP_Save Object Reference"))
  ;[0 0.09146 1] Saving System
  (set `/Game/Custom_0/Blueprints/GameplayFramework/SaveSystem/BP_Save.GameProgressionStructData` (make `/Game/Custom_0/Blueprints/GameplayFramework/SaveSystem/StructDatas/BPS_GameProgressionStruct` (`self.CurrentQuest`)) SaveGameRef))

(event `/Game/Custom_0/Blueprints/GameplayFramework/WorldProgression/BPI_UpdateWorldQuest.I_CoinCollected`
  (params (CurrentPeopleSaved :type Integer))
  ;[0.2883 1 0.212] Notify events to update Quest components and general Game scope
  ;;[1 1 1] Coin
  (bind _coincollectionquest (`self.CoinCollectionQuest`)
    (:`then`
      (`/Game/Custom_0/Blueprints/GameplayFramework/WorldProgression/Quests/QuestComponents/BP_CollectCoinQuest.CoinsUpdate` _coincollectionquest CurrentPeopleSaved))
    (:`else`)))

(event `/Game/Custom_0/Blueprints/GameplayFramework/SaveSystem/BPI_Saveable.I_LoadData`
  (params (SaveGameRef :type "/Game/Custom_0/Blueprints/GameplayFramework/SaveSystem/BP_Save Object Reference"))
  (bind _gameprogressionstructdata_currentquest (break `/Game/Custom_0/Blueprints/GameplayFramework/SaveSystem/StructDatas/BPS_GameProgressionStruct` (`/Game/Custom_0/Blueprints/GameplayFramework/SaveSystem/BP_Save.GameProgressionStructData` SaveGameRef)))
  ;[0 0.09146 1] Saving System
  (set `self.CurrentQuest` _gameprogressionstructdata_currentquest))

(event `/Game/Custom_0/Blueprints/GameplayFramework/WorldProgression/BPI_UpdateWorldQuest.I_AddMaximumCoin`
  ;[0.2883 1 0.212] Notify events to update Quest components and general Game scope
  ;;[1 1 1] Coin
  (bind _coincollectionquest (`self.CoinCollectionQuest`)
    (:`then`
      (`/Game/Custom_0/Blueprints/GameplayFramework/WorldProgression/Quests/QuestComponents/BP_CollectCoinQuest.MaxCoinIncreased` _coincollectionquest))
    (:`else`)))

(event `/Game/Custom_0/Blueprints/GameplayFramework/WorldProgression/BPI_UpdateWorldQuest.I_RemoveMaximumCoin`
  ;[0.2883 1 0.212] Notify events to update Quest components and general Game scope
  ;;[1 1 1] Coin
  (bind _coincollectionquest (`self.CoinCollectionQuest`)
    (:`then`
      (`/Game/Custom_0/Blueprints/GameplayFramework/WorldProgression/Quests/QuestComponents/BP_CollectCoinQuest.MaxCoinDecreased` _coincollectionquest))
    (:`else`)))

(event `/Game/Custom_0/Blueprints/GameplayFramework/WorldProgression/BPI_UpdateWorldQuest.I_EnemyKilled`
  ;[0.2883 1 0.212] Notify events to update Quest components and general Game scope
  ;;[1 1 1] Enemy
  (bind _killingenemiesquest (`self.KillingEnemiesQuest`)
    (:`then`
      (`/Game/Custom_0/Blueprints/GameplayFramework/WorldProgression/Quests/QuestComponents/BP_EnemyKillQuest.EnemiesUpdate` _killingenemiesquest))
    (:`else`)))

(event `/Game/Custom_0/Blueprints/GameplayFramework/WorldProgression/BPI_UpdateWorldQuest.I_EnemiesReset`
  ;[0.2883 1 0.212] Notify events to update Quest components and general Game scope
  ;;[1 1 1] Enemy
  (bind _killingenemiesquest (`self.KillingEnemiesQuest`)
    (:`then`
      (`/Game/Custom_0/Blueprints/GameplayFramework/WorldProgression/Quests/QuestComponents/BP_EnemyKillQuest.EnemiesReset` _killingenemiesquest))
    (:`else`)))

(event `/Game/Custom_0/Blueprints/GameplayFramework/WorldProgression/BPI_UpdateWorldQuest.I_PlayerGotKilled`
  ;[0.2883 1 0.212] Notify events to update Quest components and general Game scope
  ;;[1 1 1] Player
  (`self.PlayerDied`))

(event `/Game/Custom_0/Blueprints/GameplayFramework/WorldProgression/BPI_UpdateWorldQuest.I_EndConversation`
  (params (`MainQuest?` :type Boolean))
  ;[0.2883 1 0.212] Notify events to update Quest components and general Game scope
  (bind _talktonpcquest (`self.TalkToNPCQuest`)
    (:`then`
      (`/Game/Custom_0/Blueprints/GameplayFramework/WorldProgression/Quests/QuestComponents/BP_TalkToNPCQuest.QuestCompleted` _talktonpcquest `MainQuest?`))
    (:`else`)))

(fn `CheckIfAllQuestWereCompleted`
  (returns (`AllAssignedQuestCompleted?` :type Boolean))
  (return (and (`KismetArrayLibrary.Array_IsEmpty` (`self.K2_GetComponentsByClass` self "/Game/Custom_0/Blueprints/GameplayFramework/WorldProgression/Quests/QuestComponents/BP_BaseQuestComponent.BP_BaseQuestComponent_C")) (`|EnumInequality` (`self.CurrentQuest`) "NewEnumerator3"))))

(fn `CheckNewQuestParameters`
  (returns (`Out Row Quest Type` :type "/Game/Custom_0/Blueprints/GameplayFramework/WorldProgression/E_WorldQuests Enum") (`Out Row Enemies to Kill` :type Integer) (`Out Row NPCName` :type String) (`Out Row People Saved` :type Integer))
  (bind _outrownames (`DataTableFunctionLibrary.GetDataTableRowNames` "/Game/Custom_0/Blueprints/GameplayFramework/WorldProgression/Quests/DT_QuestSpecifics.DT_QuestSpecifics"))
  (bind _returnvalue (`|GetDataTableRow` "/Game/Custom_0/Blueprints/GameplayFramework/WorldProgression/Quests/DT_QuestSpecifics.DT_QuestSpecifics" (`|GetArrayItem` _outrownames (`KismetMathLibrary.Conv_ByteToInt` (`self.CurrentQuest`))))
    (:`then`
      (return (break `/Game/Custom_0/Blueprints/GameplayFramework/WorldProgression/Quests/BPS_QuestsData` _returnvalue) (`.EnemiesToKill_12_A556245742A74BBE8CA1CEB1A5F08C73` (break `/Game/Custom_0/Blueprints/GameplayFramework/WorldProgression/Quests/BPS_QuestsData` _returnvalue)) (`.NPCName_19_2C8DB01D404FD654CCA663AE42ED8444` (break `/Game/Custom_0/Blueprints/GameplayFramework/WorldProgression/Quests/BPS_QuestsData` _returnvalue)) (`.PeopleSaved_20_7BDCA2D444049FAD9EA31D9D7EE6950E` (break `/Game/Custom_0/Blueprints/GameplayFramework/WorldProgression/Quests/BPS_QuestsData` _returnvalue))))))

(fn `I_SendQuestSpecifics`
  (returns (GlobalQuestType :type "/Game/Custom_0/Blueprints/GameplayFramework/WorldProgression/E_WorldQuests Enum") (PeopleSaved :type Integer) (EnemiesToKill :type Integer) (NPCName :type String))
  (bind (_out_row_quest_type _out_row_enemies_to_kill _out_row_npcname _out_row_people_saved) (`self.CheckNewQuestParameters`))
  (return _out_row_quest_type _out_row_people_saved _out_row_enemies_to_kill _out_row_npcname))

(fn `QuestWasCompleted`
  (bind _result (`/Engine/EditorBlueprintResources/StandardMacros.IncrementInt` (`KismetMathLibrary.Conv_ByteToInt` (`self.CurrentQuest`)))
    (:`  `
      (set `self.CurrentQuest` (cast `/Game/Custom_0/Blueprints/GameplayFramework/WorldProgression/E_WorldQuests` (`KismetMathLibrary.Conv_IntToByte` _result)))
      (return))))

(fn `RemoveCurrentQuestData`
  (params (QuestTypeCompleted :type "/Game/Custom_0/Blueprints/GameplayFramework/WorldProgression/Quests/E_QuestTypes Enum" :default "NewEnumerator0"))
  (switch `/Game/Custom_0/Blueprints/GameplayFramework/WorldProgression/Quests/E_QuestTypes` QuestTypeCompleted
    (:`NewEnumerator0`
      (`ActorComponent.K2_DestroyComponent` (`self.CoinCollectionQuest`)))
    (:`NewEnumerator1`
      (`ActorComponent.K2_DestroyComponent` (`self.KillingEnemiesQuest`)))
    (:`NewEnumerator3`
      (`ActorComponent.K2_DestroyComponent` (`self.TalkToNPCQuest`)))
    (:`NewEnumerator2`
      _))
  (return))

(fn `UserConstructionScript`)