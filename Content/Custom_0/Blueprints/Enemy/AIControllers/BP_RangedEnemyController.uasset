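; AI controller for a ranged zombie enemy that runs BT_RangedZombie on possession and tracks the player through sight perception.
; Sensing a "Player"-tagged actor sets the line-of-sight flag and player reference on the Blackboard and cancels any pending reset timer.
; Losing sight starts a one-shot grace timer that clears both keys when it expires.
; BeginPlay also assigns BT_AdvancedZombie to BTAsset, though possession runs the ranged tree directly.
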(event `self.ReceiveBeginPlay`
  (set `self.BTAsset` "/Game/Custom_0/Blueprints/Enemy/AI/AdvancedWalkerEnemy/BT_AdvancedZombie.BT_AdvancedZombie"))

(event `self.ReceivePossess`
  (params (PossessedPawn :type "Pawn Object Reference"))
  ;[1 1 1] Posses the Enemy
  (set `self.Possessed Pawn` PossessedPawn)
  (`self.RunBehaviorTree` "/Game/Custom_0/Blueprints/Enemy/AI/RangedEnemy/BT_RangedZombie.BT_RangedZombie"))

(event `self.AIPerception.OnTargetPerceptionUpdated`
  (params (Actor :type "Actor Object Reference") (Stimulus :type "AIStimulus Structure"))
  ;[1 1 1] Sense Perception
  (if (`self.ActorHasTag` Actor "Player")
    (set `self.PerceivedActor` Actor)
    (bind _returnvalue (`AIPerceptionSystem.GetSenseClassForStimulus` Stimulus))
    (if (== _returnvalue "/Script/AIModule.AISense_Sight")
      (if (`.bSuccessfullySensed` (break `AIStimulus` Stimulus))
        (`KismetSystemLibrary.K2_ClearAndInvalidateTimerHandle` (`self.HasLineOfSightTimerHandle`))
        (`BlackboardComponent.SetValueAsBool` (`self.Blackboard`) (`self.VarHasLineOfSightName`) true)
        (`BlackboardComponent.SetValueAsObject` (`self.Blackboard`) (`self.VarPlayerRefName`) (`self.PerceivedActor`))
        (else
          (bind _returnvalue_2 (`KismetSystemLibrary.K2_SetTimerDelegate` (delegate `ResetSightOfPlayer`) (`self.LineOfSightDuration`)))
          (set `self.HasLineOfSightTimerHandle` _returnvalue_2))))))

(event `ResetSightOfPlayer`
  ;[1 1 1] Sense Perception
  (`BlackboardComponent.SetValueAsBool` (`self.Blackboard`) (`self.VarHasLineOfSightName`) false)
  (`BlackboardComponent.SetValueAsObject` (`self.Blackboard`) (`self.VarPlayerRefName`) null))

(fn `UserConstructionScript`
  (`parent.UserConstructionScript`))