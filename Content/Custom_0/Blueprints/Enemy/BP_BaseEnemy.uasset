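; Base enemy character with health, patrol points, item drops and player contact damage.
; Stomps, detected by hit normal, hide and unpossess it, while other contact hurts and knocks back the player; depleted health destroys it.
; Player death restores start transform and revives it unless killed before the last checkpoint.
; Save/load persists killed state by object index, and an interface serves looping patrol locations.
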(event `self.ReceiveBeginPlay`
  ;[1 1 1] BeginPlay Event
  (set `self.CurrentHealth` (`self.EnemyMaxHealth`))
  (set `self.ControllerAIRef` (`AIBlueprintHelperLibrary.GetAIController` self))
  (message `/Game/Custom_0/Blueprints/GameplayFramework/SaveSystem/BPI_Persistent.I_RequestLoad` (`GameplayStatics.GetGameInstance`) self)
  (`self.PopulateResetStruct` true)
  ;;[0 0.5493 1] Register events to reset dispatcher
  (bind _asbp_game_state_main (cast `/Game/Custom_0/Blueprints/GameplayFramework/WorldProgression/BP_GameStateMain` (`GameplayStatics.GetGameState`)))
  (add `/Game/Custom_0/Blueprints/GameplayFramework/WorldProgression/BP_GameStateMain.PlayerDied` _asbp_game_state_main (delegate `InternalReset`))
  (bind _asbp_player_state_main (cast `/Game/Custom_0/Blueprints/GameplayFramework/BP_PlayerStateMain` (`GameplayStatics.GetPlayerState` 0)))
  (add `/Game/Custom_0/Blueprints/GameplayFramework/BP_PlayerStateMain.CheckpointReached` _asbp_player_state_main (delegate `InternalCheckpointReached`)))

(event `InternalReset`
  (bind (_resetstruct_killed_ _resetstruct_starttransform) (break `/Game/Custom_0/Blueprints/GameplayFramework/ResetValuesStructs/BPS_ResetEnemy` (`self.ResetStruct`)))
  ;[1 1 1] BeginPlay Event
  ;;[0 0.5493 1] Register events to reset dispatcher
  (if (not _resetstruct_killed_)
    (`MovementComponent.StopMovementImmediately` (`self.CharacterMovement`))
    (`self.K2_SetActorTransform` self _resetstruct_starttransform false true)
    (set `self.Index` 0)
    (`self.Reset`)))

(event `InternalCheckpointReached`
  ;[1 1 1] BeginPlay Event
  ;;[0 0.5493 1] Register events to reset dispatcher
  (`self.PopulateResetStruct` false))

(event `Killed`
  (bind _returnvalue (`AIBlueprintHelperLibrary.GetAIController` self))
  ;[1 1 1] Hide enemy when Killed
  (set `self.Killed?` true)
  (`AIController.RunBehaviorTree` _returnvalue null)
  (`Controller.UnPossess` _returnvalue)
  (`PrimitiveComponent.SetCollisionEnabled` (`self.CapsuleComponent`) "NoCollision")
  (`PrimitiveComponent.SetCollisionEnabled` (`self.Hitbox`) "NoCollision")
  (`PrimitiveComponent.SetCollisionEnabled` (`self.Mesh`) "NoCollision")
  (`MovementComponent.StopMovementImmediately` (`self.CharacterMovement`))
  (`SceneComponent.SetHiddenInGame` (`self.CapsuleComponent`) true true))

(event `Reset`
  ;[1 1 1] Show and if necessary posses Enemy anew
  (if (`self.Killed?`)
    (set `self.Killed?` false)
    (message `/Game/Custom_0/Blueprints/GameplayFramework/WorldProgression/BPI_UpdateWorldQuest.I_EnemiesReset` (`GameplayStatics.GetGameState`))
    (`Controller.Possess` (`self.ControllerAIRef`) self)
    (`PrimitiveComponent.SetCollisionEnabled` (`self.CapsuleComponent`) "QueryAndPhysics")
    (`PrimitiveComponent.SetCollisionEnabled` (`self.Hitbox`) "QueryAndPhysics")
    (`PrimitiveComponent.SetCollisionEnabled` (`self.Mesh`) "QueryAndPhysics")
    (`SceneComponent.SetHiddenInGame` (`self.Mesh`) false false)))

(event `DropItem`
  ;[1 1 1] Drop Item
  (bind _output_get (set `self.DroppedItemClass` (`KismetArrayLibrary.Array_Random` (`self.DropArray`))))
  (if (`KismetSystemLibrary.IsValidClass` _output_get)
    (bind _returnvalue (`|SpawnActorFromClass` _output_get (`self.GetTransform` self) "AdjustIfPossibleButAlwaysSpawn" "MultiplyWithRoot" null null))
    (bind _asbp_pickup_base (cast `/Game/Custom_0/Blueprints/Objects/PickUpables/BP_PickupBase` _returnvalue))
    (set `/Game/Custom_0/Blueprints/Objects/PickUpables/BP_PickupBase.NeedSave?` false _asbp_pickup_base)
    (`PrimitiveComponent.SetSimulatePhysics` (`/Game/Custom_0/Blueprints/Objects/PickUpables/BP_PickupBase.Object` _asbp_pickup_base) true)))

(event `/Game/Custom_0/Blueprints/GameplayFramework/SaveSystem/BPI_Saveable.I_SaveData`
  (params (SaveGameRef :type "/Game/Custom_0/Blueprints/GameplayFramework/SaveSystem/BP_Save Object Reference"))
  ;[0.07708 0.1808 1] Saving System
  (`BlueprintMapLibrary.Map_Add` (`/Game/Custom_0/Blueprints/GameplayFramework/SaveSystem/BP_Save.EnemyStructData` SaveGameRef) (`self.ObjectIndex`) (make `/Game/Custom_0/Blueprints/GameplayFramework/SaveSystem/StructDatas/BPS_EnemyStruct` (`self.Killed?`))))

(event `/Game/Custom_0/Blueprints/GameplayFramework/SaveSystem/BPI_Saveable.I_LoadData`
  (params (SaveGameRef :type "/Game/Custom_0/Blueprints/GameplayFramework/SaveSystem/BP_Save Object Reference"))
  (bind (_value _returnvalue) (`BlueprintMapLibrary.Map_Find` (`/Game/Custom_0/Blueprints/GameplayFramework/SaveSystem/BP_Save.EnemyStructData` SaveGameRef) (`self.ObjectIndex`)))
  ;[0.07708 0.1808 1] Saving System
  (if _returnvalue
    (bind _output_get (set `self.Killed?` (break `/Game/Custom_0/Blueprints/GameplayFramework/SaveSystem/StructDatas/BPS_EnemyStruct` _value)))
    (if _output_get
      (`self.Killed`))))

(event `self.Hitbox.OnComponentBeginOverlap`
  (params (OverlappedComponent :type "PrimitiveComponent Object Reference") (OtherActor :type "Actor Object Reference") (OtherComp :type "PrimitiveComponent Object Reference") (OtherBodyIndex :type Integer) (bFromSweep :type Boolean) (SweepResult :type "HitResult Structure (by ref)"))
  (bind _returnvalue (`GameplayStatics.GetPlayerPawn` 0))
  ;[1 1 1] Player Contact Damage
  (if (`self.ActorHasTag` OtherActor "Player")
    (if (`self.CheckNormalDirection` (.z (`.Normal` (`GameplayStatics.BreakHitResult` SweepResult))))
      (`self.Killed`)
      (`self.DropItem`)
      (message `/Game/Custom_0/Blueprints/Player/BPI_PlayerUtility.I_AddRecoilImpulse` (`GameplayStatics.GetPlayerPawn` 0) (`KismetMathLibrary.Vector_Up`))
      (message `/Game/Custom_0/Blueprints/GameplayFramework/WorldProgression/BPI_UpdateWorldQuest.I_EnemyKilled` (`GameplayStatics.GetGameState`))
      (else
        (message `/Game/Custom_0/Blueprints/Player/BPI_UpdatePlayerStats.I_TakeDamage` _returnvalue)
        (message `/Game/Custom_0/Blueprints/Player/BPI_PlayerUtility.I_AddRecoilImpulse` _returnvalue (`KismetMathLibrary.Normal` (- (`self.K2_GetActorLocation` OtherActor) (`self.K2_GetActorLocation`))))))))

(event `self.I_Die`
  ;[1 1 1] Death
  (if (<= (`self.CurrentHealth`) 0.0)
    (message `/Game/Custom_0/Blueprints/GameplayFramework/WorldProgression/BPI_UpdateWorldQuest.I_EnemyKilled` (`GameplayStatics.GetGameState`))
    (`self.DropItem`)
    (`self.K2_DestroyActor` self)))

(event `self.I_TakeDamage`
  ;[1 1 1] Damage
  (set `self.CurrentHealth` (- (`self.CurrentHealth`) 20.0))
  (`self.I_Die`))

(fn `CheckNormalDirection`
  (params (Z :type "Float (double-precision)"))
  (returns (Out :type Boolean))
  (return (<= Z -0.1)))

(fn `I_SendNextPatrolLocation`
  (returns (NewPatrolLocation :type "Vector Structure"))
  ;[1 1 1] Send Next Patrol Location from Public Array
  (if (>= (`KismetArrayLibrary.Array_Length` (`self.PatrolLocations`)) 1)
    (`/Engine/EditorBlueprintResources/StandardMacros.IncrementInt` (`self.Index`)
      (:`  `
        (return (`|GetArrayItem` (`self.PatrolLocations`) (mod (+ (`self.Index`) 1) (`KismetArrayLibrary.Array_Length` (`self.PatrolLocations`)))))))))

(fn `PopulateResetStruct`
  (params (`SaveTransform?` :type Boolean))
  (bind (_resetstruct_killed_ _resetstruct_starttransform) (break `/Game/Custom_0/Blueprints/GameplayFramework/ResetValuesStructs/BPS_ResetEnemy` (`self.ResetStruct`)))
  (if `SaveTransform?`
    (set `self.ResetStruct` (make `/Game/Custom_0/Blueprints/GameplayFramework/ResetValuesStructs/BPS_ResetEnemy` (`self.Killed?`) (`self.GetTransform` self)))
    (else
      (set `self.ResetStruct` (make `/Game/Custom_0/Blueprints/GameplayFramework/ResetValuesStructs/BPS_ResetEnemy` (`self.Killed?`) _resetstruct_starttransform)))))

(fn `UserConstructionScript`)