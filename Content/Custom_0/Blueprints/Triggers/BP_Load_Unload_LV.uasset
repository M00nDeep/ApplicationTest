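; Trigger box that is meant to stream levels in when a Player-tagged actor enters and out when it leaves.
; Overlaps call CustomForEach helpers, whose visible definitions are empty or absent.
; ForEach_Load and ForEach_Unload events hold the non-blocking stream calls for the LVLoad and LVUnLoad arrays.
; Each advances a shared CurrentLevelIndex, calls its helper again while entries remain, then resets the index.
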(event `self.Box.OnComponentBeginOverlap`
  (params (OverlappedComponent :type "PrimitiveComponent Object Reference") (OtherActor :type "Actor Object Reference") (OtherComp :type "PrimitiveComponent Object Reference") (OtherBodyIndex :type Integer) (bFromSweep :type Boolean) (SweepResult :type "HitResult Structure (by ref)"))
  ;[0.09896 0.09896 0.09896 0.211] Loading Level
  (if (`self.ActorHasTag` OtherActor "Player")
    (`self.Custom_ForEach_Load`)))

(event `self.Box.OnComponentEndOverlap`
  (params (OverlappedComponent :type "PrimitiveComponent Object Reference") (OtherActor :type "Actor Object Reference") (OtherComp :type "PrimitiveComponent Object Reference") (OtherBodyIndex :type Integer))
  ;[0.09896 0.09896 0.09896 0.211] Unloading Level
  (if (`self.ActorHasTag` OtherActor "Player")
    (`self.Custom_ForEach_UnLoad`)))

(event `ForEach_Load`
  (bind _lv_load (`self.LV_Load`))
  ;[1 1 1] Custom Load Array ForEach
  (`GameplayStatics.LoadStreamLevelBySoftObjectPtr` (`|GetArrayItem` _lv_load (`self.CurrentLevel_Index`)) true)
  (set `self.CurrentLevel_Index` (+ (`self.CurrentLevel_Index`) 1))
  (if (< (`self.CurrentLevel_Index`) (`KismetArrayLibrary.Array_Length` _lv_load))
    (`self.Custom_ForEach_Load`)
    (else
      (set `self.CurrentLevel_Index` 0))))

(event `ForEach_Unload`
  (bind _lv_unload (`self.LV_UnLoad`))
  ;[1 1 1] Custom UnLoad Array ForEach
  (`GameplayStatics.UnloadStreamLevelBySoftObjectPtr` (`|GetArrayItem` _lv_unload (`self.CurrentLevel_Index`)))
  (set `self.CurrentLevel_Index` (+ (`self.CurrentLevel_Index`) 1))
  (if (< (`self.CurrentLevel_Index`) (`KismetArrayLibrary.Array_Length` _lv_unload))
    (`self.Custom_ForEach_UnLoad`)
    (else
      (set `self.CurrentLevel_Index` 0))))

(event `Custom_ForEach_UnLoad`)

(fn `Custom_ForEach_Load`)

(fn `UserConstructionScript`)