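; BP_TutorialTrigger is a one-shot trigger volume that shows the player a timed tutorial message.
; When an actor tagged Player begins overlapping its Box, a DoOnce gate lets the first overlap create a WBP_Tutorial widget with TutorialText and add it to the viewport.
; After TextDuration it removes the widget and destroys itself.
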(event `self.Box.OnComponentBeginOverlap`
  (params (OverlappedComponent :type "PrimitiveComponent Object Reference") (OtherActor :type "Actor Object Reference") (OtherComp :type "PrimitiveComponent Object Reference") (OtherBodyIndex :type Integer) (bFromSweep :type Boolean) (SweepResult :type "HitResult Structure (by ref)"))
  (if (`self.ActorHasTag` OtherActor "Player")
    (`/Engine/EditorBlueprintResources/StandardMacros.DoOnce` false
      (:`Completed`
        (bind _returnvalue (`|CreateWidget` "/Game/Custom_0/Blueprints/Widgets/Tutorials/WBP_Tutorial.WBP_Tutorial_C"))
        (`TextBlock.SetText` (`/Game/Custom_0/Blueprints/Widgets/Tutorials/WBP_Tutorial.TextTutorial` _returnvalue) (`KismetTextLibrary.Conv_StringToText` (`self.TutorialText`)))
        (`UserWidget.AddToViewport` _returnvalue 0)
        (`KismetSystemLibrary.Delay` (`self.TextDuration`))
        (`Widget.RemoveFromParent` _returnvalue)
        (`self.K2_DestroyActor`)))))

(fn `UserConstructionScript`)