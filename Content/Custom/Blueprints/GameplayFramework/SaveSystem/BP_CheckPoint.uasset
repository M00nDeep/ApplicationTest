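; BP_CheckPoint is a one-time checkpoint that requests a game save when an actor tagged Player overlaps its box.
; On use it marks itself used, turns the flag material green and destroys the trigger box.
; At BeginPlay it requests a load through the game instance interface.
; Its save and load interface events store the used flag by ObjectIndex in the save's TriggerStructData map, so used checkpoints restore as used.
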(event `self.ReceiveBeginPlay`
  (message `/Game/Custom/Blueprints/GameplayFramework/SaveSystem/BPI_Persistent.I_RequestLoad` (`GameplayStatics.GetGameInstance`) self))

(event `self.Box.OnComponentBeginOverlap`
  (params (OverlappedComponent :type "PrimitiveComponent Object Reference") (OtherActor :type "Actor Object Reference") (OtherComp :type "PrimitiveComponent Object Reference") (OtherBodyIndex :type Integer) (bFromSweep :type Boolean) (SweepResult :type "HitResult Structure (by ref)"))
  (if (`self.ActorHasTag` OtherActor "Player")
    (`self.CheckpointUsed`)
    (message `/Game/Custom/Blueprints/GameplayFramework/SaveSystem/BPI_Persistent.I_RequestSave` (`GameplayStatics.GetGameInstance`) true)))

(event `/Game/Custom/Blueprints/GameplayFramework/SaveSystem/BPI_Saveable.I_SaveData`
  (params (SaveGameRef :type "/Game/Custom/Blueprints/GameplayFramework/SaveSystem/BP_Save Object Reference"))
  (`BlueprintMapLibrary.Map_Add` (`/Game/Custom/Blueprints/GameplayFramework/SaveSystem/BP_Save.TriggerStructData` SaveGameRef) (`self.ObjectIndex`) (make `/Game/Custom/Blueprints/GameplayFramework/SaveSystem/StructDatas/BPS_TriggerStruct` (`self.AlreadyUsed`))))

(event `/Game/Custom/Blueprints/GameplayFramework/SaveSystem/BPI_Saveable.I_LoadData`
  (params (SaveGameRef :type "/Game/Custom/Blueprints/GameplayFramework/SaveSystem/BP_Save Object Reference"))
  (bind (_value _returnvalue) (`BlueprintMapLibrary.Map_Find` (`/Game/Custom/Blueprints/GameplayFramework/SaveSystem/BP_Save.TriggerStructData` SaveGameRef) (`self.ObjectIndex`)))
  (if _returnvalue
    (bind _output_get (set `self.AlreadyUsed` (break `/Game/Custom/Blueprints/GameplayFramework/SaveSystem/StructDatas/BPS_TriggerStruct` _value)))
    (if _output_get
      (`self.CheckpointUsed`))))

(fn `CheckpointUsed`
  (set `self.AlreadyUsed` true)
  (`PrimitiveComponent.SetMaterial` (`self.Flag`) 0 "/Game/Custom/Assets/Materials/M_Green.M_Green")
  (`ActorComponent.K2_DestroyComponent` (`self.Box`))
  (return))

(fn `UserConstructionScript`)