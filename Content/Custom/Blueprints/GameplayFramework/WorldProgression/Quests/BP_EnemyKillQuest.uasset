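; BP_EnemyKillQuest is a world progression quest that completes once a required number of enemies are killed.
; BeginPlay sets its quest type and kill target, and EnemiesUpdate increments the kill counter.
; CheckQuestCompletition is a separate event that compares the counter to the target and, when met, reports the quest type to BP_GameStateMain through QuestCompleted.
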(event `self.ReceiveBeginPlay`
  (set `self.QuestType` "NewEnumerator1")
  (set `self.EnemiesToKill` 2))

(event `EnemiesUpdate`
  (`/Engine/EditorBlueprintResources/StandardMacros.IncrementInt` (`self.CurrentEnemiesKilled`)))

(event `self.CheckQuestCompletition`
  (if (>= (`self.CurrentEnemiesKilled`) (`self.EnemiesToKill`))
    (bind _asbp_game_state_main (cast `/Game/Custom/Blueprints/GameplayFramework/WorldProgression/BP_GameStateMain` (`GameplayStatics.GetGameState`)))
    (`/Game/Custom/Blueprints/GameplayFramework/WorldProgression/BP_GameStateMain.QuestCompleted` _asbp_game_state_main (`self.QuestType`))))