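; Quest component for the coin-collection quest, which tracks collected coins against a target and shows progress on a quest HUD widget.
; On BeginPlay it gets the target from the game state through an interface message, then adds the coin HUD widget.
; Coin events update the current count or raise the target by one, pushing changes to the widget.
; Reaching the target removes the widget and reports completion to BP_GameStateMain.
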(event `self.ReceiveBeginPlay`
  (`|ExecutionSequence`
    (:`then_0`
      (set `self.QuestType` "NewEnumerator0")
      (bind (_globalquesttype _coinstocollect) (message `/Game/Custom/Blueprints/GameplayFramework/WorldProgression/BPI_UpdateWorldQuest.I_SendQuestSpecifics` (`GameplayStatics.GetGameState`)))
      (set `self.CoinsToCollect` _coinstocollect)
      (set `self.WidgetClass` "/Game/Custom/Blueprints/Widgets/WBP_CoinQuestHUD.WBP_CoinQuestHUD_C"))
    (:`then_1`
      (`self.AddQuestWidget` self)
      (message `/Game/Custom/Blueprints/Widgets/BPI_SendDataToWidget.I_SendTotalCoinsQuest` (`self.WidgetRef`) (`self.CoinsToCollect`)))))

(event `CoinsUpdate`
  (params (CoinsToCollect :type Integer))
  (set `self.CurrentCoinsCollected` CoinsToCollect)
  (message `/Game/Custom/Blueprints/Widgets/BPI_SendDataToWidget.I_SendCurrentCoinsQuest` (`self.WidgetRef`) (`self.CurrentCoinsCollected`))
  (`self.CheckQuestCompletition`))

(event `MaxCoinUpdated`
  (`/Engine/EditorBlueprintResources/StandardMacros.IncrementInt` (`self.CoinsToCollect`)
    (:`  `
      (message `/Game/Custom/Blueprints/Widgets/BPI_SendDataToWidget.I_SendTotalCoinsQuest` (`self.WidgetRef`) (`self.CoinsToCollect`)))))

(event `self.CheckQuestCompletition`
  (if (>= (`self.CurrentCoinsCollected`) (`self.CoinsToCollect`))
    (`self.RemoveQuestWidget`)
    (bind _asbp_game_state_main (cast `/Game/Custom/Blueprints/GameplayFramework/WorldProgression/BP_GameStateMain` (`GameplayStatics.GetGameState`)))
    (`/Game/Custom/Blueprints/GameplayFramework/WorldProgression/BP_GameStateMain.QuestCompleted` _asbp_game_state_main (`self.QuestType`))))