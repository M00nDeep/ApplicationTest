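; BP_CollectCoinQuest is a quest that completes once enough coins are collected, with the target set to two on BeginPlay.
; CoinsUpdate overwrites the collected count with the value passed in, then runs the completion check.
; When the count reaches or exceeds the target, the check casts the game state to BP_GameStateMain and calls QuestCompleted on it.
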(event `self.ReceiveBeginPlay`
  (set `self.CoinsToCollect` 2))

(event `CoinsUpdate`
  (params (CoinsToCollect :type Integer))
  (set `self.CurrentCoinsCollected` CoinsToCollect)
  (`self.CheckQuestCompletition`))

(event `CheckQuestCompletition`
  (if (>= (`self.CurrentCoinsCollected`) (`self.CoinsToCollect`))
    (bind _asbp_game_state_main (cast `/Game/Custom/Blueprints/GameplayFramework/WorldProgression/BP_GameStateMain` (`GameplayStatics.GetGameState`)))
    (`/Game/Custom/Blueprints/GameplayFramework/WorldProgression/BP_GameStateMain.QuestCompleted` _asbp_game_state_main)))