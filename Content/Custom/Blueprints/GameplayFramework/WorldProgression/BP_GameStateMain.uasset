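; Main GameState that drives world quest progression through an enum of quest stages, ending the game at the final stage.
; Each stage spawns coin-collection and/or enemy-kill quest components, which receive updates through interface events.
; Completed quests destroy their component; when no quest components remain, it broadcasts progression, increments the enum and sets up the next stage.
; The current quest is loaded on BeginPlay and saved through save/load interface events.
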(event `DefineCurrentQuest`
  (params (CurrentQuest :type "/Game/Custom/Blueprints/GameplayFramework/WorldProgression/E_WorldQuests Enum" :default "NewEnumerator0"))
  ;[1 1 1] Assign Correct quests based on Enum
  (switch `/Game/Custom/Blueprints/GameplayFramework/WorldProgression/E_WorldQuests` CurrentQuest
    (:`NewEnumerator0`
      (bind _returnvalue (`AddComponent|NODE_AddBP_CollectCoinQuest-0`))
      (set `self.CoinCollectionQuest` _returnvalue))
    (:`NewEnumerator1`
      (bind _returnvalue_2 (`AddComponent|NODE_AddBP_EnemyKillQuest-0`))
      (set `self.KillingEnemiesQuest` _returnvalue_2))
    (:`NewEnumerator2`
      (bind _returnvalue_3 (`AddComponent|NODE_AddBP_CollectCoinQuest-1`))
      (set `self.CoinCollectionQuest` _returnvalue_3)
      (bind _returnvalue_4 (`AddComponent|NODE_AddBP_EnemyKillQuest-1`))
      (set `self.KillingEnemiesQuest` _returnvalue_4))
    (:`NewEnumerator3`
      (`self.EndGame`))))

(event `self.ReceiveBeginPlay`
  ;[1 1 1] Begin Play - Load Current Quest and Define it
  (message `/Game/Custom/Blueprints/GameplayFramework/SaveSystem/BPI_Persistent.I_RequestLoad` (`GameplayStatics.GetGameInstance`) self)
  (`self.DefineCurrentQuest` (`self.CurrentQuest`)))

(event `QuestCompleted`
  (params (QuestTypeCompleted :type "/Game/Custom/Blueprints/GameplayFramework/WorldProgression/Quests/E_QuestTypes Enum" :default "NewEnumerator0"))
  ;[1 1 1] Quest was completes - notify everyone and remove relative component
  (`self.RemoveCurrentQuestData` QuestTypeCompleted)
  (bind _allassignedquestcompleted_ (`self.CheckIfAllQuestWereCompleted`))
  (if _allassignedquestcompleted_
    (`self.QuestProgression` (`self.CurrentQuest`))
    (`self.QuestWasCompleted`)
    (`self.DefineCurrentQuest` (`self.CurrentQuest`))))

(event `/Game/Custom/Blueprints/GameplayFramework/SaveSystem/BPI_Saveable.I_SaveData`
  (params (SaveGameRef :type "/Game/Custom/Blueprints/GameplayFramework/SaveSystem/BP_Save Object Reference"))
  ;[0 0.09146 1] Saving System
  (set `/Game/Custom/Blueprints/GameplayFramework/SaveSystem/BP_Save.GameProgressionStructData` (make `/Game/Custom/Blueprints/GameplayFramework/SaveSystem/StructDatas/BPS_GameProgressionStruct` (`self.CurrentQuest`)) SaveGameRef))

(event `/Game/Custom/Blueprints/GameplayFramework/WorldProgression/BPI_UpdateWorldQuest.I_CoinCollected`
  (params (CurrentCoinsCollected :type Integer))
  ;[0.2883 1 0.212] Notify events to update Quest components
  ;;[1 1 1] Coin
  (`/Game/Custom/Blueprints/GameplayFramework/WorldProgression/Quests/BP_CollectCoinQuest.CoinsUpdate` (`self.CoinCollectionQuest`) CurrentCoinsCollected))

(event `/Game/Custom/Blueprints/GameplayFramework/SaveSystem/BPI_Saveable.I_LoadData`
  (params (SaveGameRef :type "/Game/Custom/Blueprints/GameplayFramework/SaveSystem/BP_Save Object Reference"))
  (bind _gameprogressionstructdata_currentquest (break `/Game/Custom/Blueprints/GameplayFramework/SaveSystem/StructDatas/BPS_GameProgressionStruct` (`/Game/Custom/Blueprints/GameplayFramework/SaveSystem/BP_Save.GameProgressionStructData` SaveGameRef)))
  ;[0 0.09146 1] Saving System
  (set `self.CurrentQuest` _gameprogressionstructdata_currentquest))

(event `/Game/Custom/Blueprints/GameplayFramework/WorldProgression/BPI_UpdateWorldQuest.I_AddMaximumCoin`
  ;[0.2883 1 0.212] Notify events to update Quest components
  ;;[1 1 1] Coin
  (`/Game/Custom/Blueprints/GameplayFramework/WorldProgression/Quests/BP_CollectCoinQuest.MaxCoinUpdated` (`self.CoinCollectionQuest`)))

(event `/Game/Custom/Blueprints/GameplayFramework/WorldProgression/BPI_UpdateWorldQuest.I_EnemyKilled`
  ;[0.2883 1 0.212] Notify events to update Quest components
  ;;[1 1 1] Enemy
  (`/Game/Custom/Blueprints/GameplayFramework/WorldProgression/Quests/BP_EnemyKillQuest.EnemiesUpdate` (`self.KillingEnemiesQuest`)))

(fn `CheckIfAllQuestWereCompleted`
  (returns (`AllAssignedQuestCompleted?` :type Boolean))
  (return (and (`KismetArrayLibrary.Array_IsEmpty` (`self.K2_GetComponentsByClass` self "/Game/Custom/Blueprints/GameplayFramework/WorldProgression/Quests/BP_BaseQuestComponent.BP_BaseQuestComponent_C")) (`|EnumInequality` (`self.CurrentQuest`) "NewEnumerator3"))))

(fn `QuestWasCompleted`
  (bind _result (`/Engine/EditorBlueprintResources/StandardMacros.IncrementInt` (`KismetMathLibrary.Conv_ByteToInt` (`self.CurrentQuest`)))
    (:`  `
      (set `self.CurrentQuest` (cast `/Game/Custom/Blueprints/GameplayFramework/WorldProgression/E_WorldQuests` (`KismetMathLibrary.Conv_IntToByte` _result)))
      (return))))

(fn `RemoveCurrentQuestData`
  (params (QuestTypeCompleted :type "/Game/Custom/Blueprints/GameplayFramework/WorldProgression/Quests/E_QuestTypes Enum" :default "NewEnumerator0"))
  (switch `/Game/Custom/Blueprints/GameplayFramework/WorldProgression/Quests/E_QuestTypes` QuestTypeCompleted
    (:`NewEnumerator0`
      (`ActorComponent.K2_DestroyComponent` (`self.CoinCollectionQuest`)))
    (:`NewEnumerator1`
      (`ActorComponent.K2_DestroyComponent` (`self.KillingEnemiesQuest`))))
  (return))

(fn `UserConstructionScript`)