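; BP_CloudPlatform is a cloud platform that switches its solidity based on the direction from which the player touches it.
; When an actor tagged Player begins overlapping its Box, CheckNormalDirection tests whether the sweep's impact normal points almost straight up along Z.
; A match disables the static mesh's collision, while any other direction restores query and physics collision.
; Nothing resets collision when the overlap ends.
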(event `self.Box.OnComponentBeginOverlap`
  (params (OverlappedComponent :type "PrimitiveComponent Object Reference") (OtherActor :type "Actor Object Reference") (OtherComp :type "PrimitiveComponent Object Reference") (OtherBodyIndex :type Integer) (bFromSweep :type Boolean) (SweepResult :type "HitResult Structure (by ref)"))
  ;[1 1 1] Begin Overlap with Box and manage cloud collision
  (if (`self.ActorHasTag` OtherActor "Player")
    (if (`self.CheckNormalDirection` (.x (`.ImpactNormal` (`GameplayStatics.BreakHitResult` SweepResult))) (.y (`.ImpactNormal` (`GameplayStatics.BreakHitResult` SweepResult))) (.z (`.ImpactNormal` (`GameplayStatics.BreakHitResult` SweepResult))))
      (`PrimitiveComponent.SetCollisionEnabled` (`self.StaticMesh`) "NoCollision")
      (else
        (`PrimitiveComponent.SetCollisionEnabled` (`self.StaticMesh`) "QueryAndPhysics")))))

(fn `CheckNormalDirection`
  (params (X :type "Float (double-precision)") (Y :type "Float (double-precision)") (Z :type "Float (double-precision)"))
  (returns (Out :type Boolean))
  ;[1 1 1] Evaluate correct direction of collision
  (return (and (<= (`KismetMathLibrary.Abs` X) 0.1) (<= (`KismetMathLibrary.Abs` Y) 0.1) (>= Z 0.1))))

(fn `UserConstructionScript`)