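; End-game trigger that opens a configured level when the player overlaps its box, once it has been activated.
; It starts with its text hidden, then becomes usable and shows the text when the game state fires its EndGame event.
; The usable flag is saved by object index and restored on load, so the exit stays active if the player quits before using it.
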(event `self.ReceiveBeginPlay`
  ;[1 1 1] Save EndGame Trigger because player could close application in front of it
  (`SceneComponent.SetVisibility` (`self.TextRender`) false false)
  (message `/Game/Custom/Blueprints/GameplayFramework/SaveSystem/BPI_Persistent.I_RequestLoad` (`GameplayStatics.GetGameInstance`) self)
  ;[0.2081 0.5332 1] Bind to End Game Call
  (bind _asbp_game_state_main (cast `/Game/Custom/Blueprints/GameplayFramework/WorldProgression/BP_GameStateMain` (`GameplayStatics.GetGameState`)))
  (add `/Game/Custom/Blueprints/GameplayFramework/WorldProgression/BP_GameStateMain.EndGame` _asbp_game_state_main (delegate `EndGameCalled`)))

(event `EndGameCalled`
  ;[0.2081 0.5332 1] Bind to End Game Call
  (set `self.CanBeUsed` true)
  (`SceneComponent.SetVisibility` (`self.TextRender`) true false))

(event `self.Box.OnComponentBeginOverlap`
  (params (OverlappedComponent :type "PrimitiveComponent Object Reference") (OtherActor :type "Actor Object Reference") (OtherComp :type "PrimitiveComponent Object Reference") (OtherBodyIndex :type Integer) (bFromSweep :type Boolean) (SweepResult :type "HitResult Structure (by ref)"))
  ;[1 1 1] open New Level
  (if (and (`self.ActorHasTag` OtherActor "Player") (`self.CanBeUsed`))
    (`GameplayStatics.OpenLevelBySoftObjectPtr` (`self.LevelToOpen`))))

(event `/Game/Custom/Blueprints/GameplayFramework/SaveSystem/BPI_Saveable.I_SaveData`
  (params (SaveGameRef :type "/Game/Custom/Blueprints/GameplayFramework/SaveSystem/BP_Save Object Reference"))
  ;[0.03692 0.179 1] Save System
  (`BlueprintMapLibrary.Map_Add` (`/Game/Custom/Blueprints/GameplayFramework/SaveSystem/BP_Save.TriggerStructData` SaveGameRef) (`self.Object Index`) (make `/Game/Custom/Blueprints/GameplayFramework/SaveSystem/StructDatas/BPS_TriggerStruct` (`self.CanBeUsed`))))

(event `/Game/Custom/Blueprints/GameplayFramework/SaveSystem/BPI_Saveable.I_LoadData`
  (params (SaveGameRef :type "/Game/Custom/Blueprints/GameplayFramework/SaveSystem/BP_Save Object Reference"))
  (bind (_value _returnvalue) (`BlueprintMapLibrary.Map_Find` (`/Game/Custom/Blueprints/GameplayFramework/SaveSystem/BP_Save.TriggerStructData` SaveGameRef) (`self.Object Index`)))
  ;[0.03692 0.179 1] Save System
  (if _returnvalue
    (bind _output_get (set `self.CanBeUsed` (break `/Game/Custom/Blueprints/GameplayFramework/SaveSystem/StructDatas/BPS_TriggerStruct` _value)))
    (if _output_get
      (`SceneComponent.SetVisibility` (`self.TextRender`) true false))))

(fn `UserConstructionScript`)