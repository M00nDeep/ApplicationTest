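; BP_Projectile is a fire projectile that flies at the player and deals damage and knockback on impact.
; On BeginPlay it locks a direction toward the player character's current position and attaches a fire particle effect.
; Tick moves it in a straight line with a swept SetActorLocation, so it does not home.
; Any hit destroys it; Player-tagged actors first trigger damage and recoil-impulse interface messages on the player pawn.
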(event `self.ReceiveBeginPlay`
  (set `self.Direction` (`KismetMathLibrary.Normal` (- (`self.K2_GetActorLocation` (`GameplayStatics.GetPlayerCharacter` 0)) (`self.K2_GetActorLocation`))))
  (`GameplayStatics.SpawnEmitterAttached` "/Game/ThirdPersonTemplate/StarterContent/Particles/P_Fire.P_Fire" (`self.Projectile`) "None" (0.0 0.0 0.0) (struct) (0.2 0.2 0.2) "SnapToTarget"))

(event `self.ReceiveTick`
  (params (DeltaSeconds :type "Float (single-precision)"))
  (`self.K2_SetActorLocation` (+ (`self.K2_GetActorLocation`) (* (`self.Direction`) (* DeltaSeconds (`self.Speed`)))) true))

(event `self.Projectile.OnComponentHit`
  (params (HitComponent :type "PrimitiveComponent Object Reference") (OtherActor :type "Actor Object Reference") (OtherComp :type "PrimitiveComponent Object Reference") (NormalImpulse :type "Vector Structure") (Hit :type "HitResult Structure (by ref)"))
  (bind _returnvalue (`GameplayStatics.GetPlayerPawn` 0))
  (if (`self.ActorHasTag` OtherActor "Player")
    (message `/Game/Custom/Blueprints/Player/BPI_UpdatePlayerStats.I_TakeDamage` _returnvalue)
    (message `/Game/Custom/Blueprints/Player/BPI_PlayerUtility.I_AddRecoilImpulse` _returnvalue (`KismetMathLibrary.Normal` (- (`self.K2_GetActorLocation` OtherActor) (`self.K2_GetActorLocation`))))
    (`self.K2_DestroyActor` self)
    (else
      (`self.K2_DestroyActor` self))))

(fn `UserConstructionScript`)