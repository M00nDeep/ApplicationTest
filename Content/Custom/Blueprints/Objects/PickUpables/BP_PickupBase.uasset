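; BP_PickupBase is a base Blueprint for collectible objects that remember whether they were collected across saves.
; A Box overlap by an actor tagged Player calls PickUp, which sets the PickedUp flag.
; On BeginPlay it asks the GameInstance to load, and it saves and restores the flag in the save game's pickup map keyed by ObjectIndex.
; Loading a collected state fires AlreadyPickedUp, an empty event here.
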(event `self.ReceiveBeginPlay`
  (message `/Game/Custom/Blueprints/GameplayFramework/SaveSystem/BPI_Persistent.I_RequestLoad` (`GameplayStatics.GetGameInstance`) self))

(event `PickUp`
  (set `self.PickedUp` true))

(event `AlreadyPickedUp`)

(event `self.Box.OnComponentBeginOverlap`
  (params (OverlappedComponent :type "PrimitiveComponent Object Reference") (OtherActor :type "Actor Object Reference") (OtherComp :type "PrimitiveComponent Object Reference") (OtherBodyIndex :type Integer) (bFromSweep :type Boolean) (SweepResult :type "HitResult Structure (by ref)"))
  (if (`self.ActorHasTag` OtherActor "Player")
    (`self.PickUp`)))

(event `/Game/Custom/Blueprints/GameplayFramework/SaveSystem/BPI_Saveable.I_SaveData`
  (params (SaveGameRef :type "/Game/Custom/Blueprints/GameplayFramework/SaveSystem/BP_Save Object Reference"))
  (`BlueprintMapLibrary.Map_Add` (`/Game/Custom/Blueprints/GameplayFramework/SaveSystem/BP_Save.PickupStructData` SaveGameRef) (`self.ObjectIndex`) (make `/Game/Custom/Blueprints/GameplayFramework/SaveSystem/StructDatas/BPS_PickupData` (`self.PickedUp`))))

(event `/Game/Custom/Blueprints/GameplayFramework/SaveSystem/BPI_Saveable.I_LoadData`
  (params (SaveGameRef :type "/Game/Custom/Blueprints/GameplayFramework/SaveSystem/BP_Save Object Reference"))
  (bind (_value _returnvalue) (`BlueprintMapLibrary.Map_Find` (`/Game/Custom/Blueprints/GameplayFramework/SaveSystem/BP_Save.PickupStructData` SaveGameRef) (`self.ObjectIndex`)))
  (if _returnvalue
    (bind _output_get (set `self.PickedUp` (break `/Game/Custom/Blueprints/GameplayFramework/SaveSystem/StructDatas/BPS_PickupData` _value)))
    (if _output_get
      (`self.AlreadyPickedUp`))))

(fn `UserConstructionScript`)