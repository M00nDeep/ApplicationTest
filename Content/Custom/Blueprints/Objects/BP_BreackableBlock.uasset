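; Breakable block that drops a random pickup from DropArray when the player's overlap has a vertical, positive-Z impact normal.
; Drops spawn above the box with physics on and saving off for pickups, and dropped coins notify the GameState to raise the maximum coin count.
; Breaking hides the mesh and disables collision after a delay.
; Broken state is saved by ObjectIndex and reapplied on load, requested at BeginPlay.
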(event `self.ReceiveBeginPlay`
  (message `/Game/Custom/Blueprints/GameplayFramework/SaveSystem/BPI_Persistent.I_RequestLoad` (`GameplayStatics.GetGameInstance`) self))

(event `DropItem`
  (bind _outitem (`KismetArrayLibrary.Array_Random` (`self.DropArray`)))
  (if (`KismetSystemLibrary.IsValidClass` _outitem)
    (bind _returnvalue (`|SpawnActorFromClass` _outitem (`self.SpawnObjectFuncUtility`) "AdjustIfPossibleButAlwaysSpawn" "MultiplyWithRoot" null (`GameplayStatics.GetPlayerPawn` 0)))
    (`self.CheckForMoreCoins` _returnvalue)
    (bind _asbp_pickup_base (cast `/Game/Custom/Blueprints/Objects/PickUpables/BP_PickupBase` _returnvalue))
    (set `/Game/Custom/Blueprints/Objects/PickUpables/BP_PickupBase.NeedSave?` false _asbp_pickup_base)
    (`PrimitiveComponent.SetSimulatePhysics` (`/Game/Custom/Blueprints/Objects/PickUpables/BP_PickupBase.Object` _asbp_pickup_base) true)))

(event `DestroyBlock`
  (`PrimitiveComponent.SetSimulatePhysics` (`self.StaticMesh`) false)
  (`SceneComponent.SetHiddenInGame` (`self.StaticMesh`) true true)
  (`KismetSystemLibrary.Delay` (`self.Duration`))
  (`PrimitiveComponent.SetCollisionEnabled` (`self.Box`) "NoCollision")
  (`PrimitiveComponent.SetCollisionEnabled` (`self.StaticMesh`) "NoCollision"))

(event `self.Box.OnComponentBeginOverlap`
  (params (OverlappedComponent :type "PrimitiveComponent Object Reference") (OtherActor :type "Actor Object Reference") (OtherComp :type "PrimitiveComponent Object Reference") (OtherBodyIndex :type Integer) (bFromSweep :type Boolean) (SweepResult :type "HitResult Structure (by ref)"))
  (if (`self.ActorHasTag` OtherActor "Player")
    (if (`self.CheckNormalDirection` (.x (`.ImpactNormal` (`GameplayStatics.BreakHitResult` SweepResult))) (.y (`.ImpactNormal` (`GameplayStatics.BreakHitResult` SweepResult))) (.z (`.ImpactNormal` (`GameplayStatics.BreakHitResult` SweepResult))))
      (set `self.AlreadyBroken` true)
      (`self.DropItem`)
      (`self.DestroyBlock`))))

(event `/Game/Custom/Blueprints/GameplayFramework/SaveSystem/BPI_Saveable.I_SaveData`
  (params (SaveGameRef :type "/Game/Custom/Blueprints/GameplayFramework/SaveSystem/BP_Save Object Reference"))
  (`BlueprintMapLibrary.Map_Add` (`/Game/Custom/Blueprints/GameplayFramework/SaveSystem/BP_Save.BlockStructData` SaveGameRef) (`self.ObjectIndex`) (make `/Game/Custom/Blueprints/GameplayFramework/SaveSystem/StructDatas/BPS_BlocksStruct` (`self.AlreadyBroken`))))

(event `/Game/Custom/Blueprints/GameplayFramework/SaveSystem/BPI_Saveable.I_LoadData`
  (params (SaveGameRef :type "/Game/Custom/Blueprints/GameplayFramework/SaveSystem/BP_Save Object Reference"))
  (bind (_value _returnvalue) (`BlueprintMapLibrary.Map_Find` (`/Game/Custom/Blueprints/GameplayFramework/SaveSystem/BP_Save.BlockStructData` SaveGameRef) (`self.ObjectIndex`)))
  (if _returnvalue
    (bind _output_get (set `self.AlreadyBroken` (break `/Game/Custom/Blueprints/GameplayFramework/SaveSystem/StructDatas/BPS_BlocksStruct` _value)))
    (if _output_get
      (`self.DestroyBlock`))))

(fn `CheckNormalDirection`
  (params (X :type "Float (double-precision)") (Y :type "Float (double-precision)") (Z :type "Float (double-precision)"))
  (returns (Out :type Boolean))
  (return (and (<= (`KismetMathLibrary.Abs` X) 0.1) (<= (`KismetMathLibrary.Abs` Y) 0.1) (>= Z 0.1))))

(fn `SpawnObjectFuncUtility`
  (returns (ReturnValue :type "Transform Structure"))
  (bind (_returnvalue_x _returnvalue_y _returnvalue_z) (`KismetMathLibrary.BreakVector` (`SceneComponent.K2_GetComponentLocation` (`self.Box`))))
  (return (`KismetMathLibrary.MakeTransform` (`KismetMathLibrary.MakeVector` _returnvalue_x _returnvalue_y (+ _returnvalue_z (`self.ZOffset`))) (`self.K2_GetActorRotation`))))

(fn `UserConstructionScript`)